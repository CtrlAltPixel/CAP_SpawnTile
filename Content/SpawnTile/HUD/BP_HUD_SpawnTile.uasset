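; HUD Blueprint for SpawnTile that puts the HUD widget on screen and controls its death overlay.
; On BeginPlay it creates WB_HUD_SpawnTile, stores the reference and adds it to the viewport.
; ShowDeadOverlay and RemoveDeadOverlay check that the widget is valid, then set or clear the IsDead flag on its nested dead overlay widget.
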(event `self.ReceiveBeginPlay`
  (bind _returnvalue (`|CreateWidget` "/Game/SpawnTile/HUD/WB_HUD_SpawnTile.WB_HUD_SpawnTile_C"))
  (bind _output_get (set `self.AsWBHUDSpawnTile` _returnvalue))
  (`UserWidget.AddToViewport` _output_get 0))

(fn `RemoveDeadOverlay`
  (bind _aswbhudspawntile (`self.AsWBHUDSpawnTile`)
    (:`then`
      (set `/Game/SpawnTile/HUD/WB_HUD_DeadOverlay.bIsDead?` false (`/Game/SpawnTile/HUD/WB_HUD_SpawnTile.WB_HUD_DeadOverlay` _aswbhudspawntile)))
    (:`else`)))

(fn `ShowDeadOverlay`
  (bind _aswbhudspawntile (`self.AsWBHUDSpawnTile`)
    (:`then`
      (set `/Game/SpawnTile/HUD/WB_HUD_DeadOverlay.bIsDead?` true (`/Game/SpawnTile/HUD/WB_HUD_SpawnTile.WB_HUD_DeadOverlay` _aswbhudspawntile)))
    (:`else`)))

(fn `UserConstructionScript`)