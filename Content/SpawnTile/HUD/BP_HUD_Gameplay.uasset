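; BP_HUD_Gameplay is the gameplay HUD that creates the WB_HUD_SpawnTile widget and toggles its dead overlay.
; BeginPlay caches player controller 0 as BP_PC_Gameplay, then adds the widget to the viewport.
; Show and Hide events set the overlay's visibility with optional debug prints, but appear inverted: Show collapses it and Hide makes it HitTestInvisible.
; Both debug messages read "Show Death Screen".
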(event `self.ReceiveBeginPlay`
  (`self.InitCasts`)
  (bind _returnvalue (`|CreateWidget` "/Game/SpawnTile/HUD/WB_HUD_SpawnTile.WB_HUD_SpawnTile_C"))
  (set `self.AsWBHUDSpawnTile` _returnvalue)
  (`UserWidget.AddToViewport` (`self.AsWBHUDSpawnTile`) 0))

(event `EventHUDShowDeadOverlay`
  (`|ExecutionSequence`
    (:`then_0`
      (if (`self.bShowDebug?`)
        (`KismetSystemLibrary.PrintString` "BP_HUD_Gameplay - Show Death Screen")))
    (:`then_1`
      (bind _aswbhudspawntile (`self.AsWBHUDSpawnTile`)
        (:`then`
          (set `Widget.Visibility` "Collapsed" (`/Game/SpawnTile/HUD/WB_HUD_SpawnTile.WB_HUD_DeadOverlay` _aswbhudspawntile)))
        (:`else`)))))

(event `EventHUDHideDeadOverlay`
  (`|ExecutionSequence`
    (:`then_0`
      (if (`self.bShowDebug?`)
        (`KismetSystemLibrary.PrintString` "BP_HUD_Gameplay - Show Death Screen")))
    (:`then_1`
      (bind _aswbhudspawntile (`self.AsWBHUDSpawnTile`)
        (:`then`
          (set `Widget.Visibility` "HitTestInvisible" (`/Game/SpawnTile/HUD/WB_HUD_SpawnTile.WB_HUD_DeadOverlay` _aswbhudspawntile)))
        (:`else`)))))

(fn `InitCasts`
  (bind _asbp_pc_gameplay (cast `/Game/SpawnTile/Player/Controller/BP_PC_Gameplay` (`GameplayStatics.GetPlayerController` 0)))
  (set `self.AsLocalPlayerController` _asbp_pc_gameplay))

(fn `UserConstructionScript`)