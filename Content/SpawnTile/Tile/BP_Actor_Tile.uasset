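; Spawn tile actor that a player selects to set a spawn point through BP_PS_SpawnTile on their PlayerState.
; Interaction lets one controller claim the tile or deselect its own, while separate set and remove functions call SERVERActionSpawn, with or without the arrow's relative transform.
; The selection RepNotify applies the same orange in both branches to an unnamed material parameter.
; ShowSpawnTile hides the cube and HideSpawnTile reveals it.
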(event `self.ReceiveBeginPlay`)

(fn `HideSpawnTile`
  (`SceneComponent.SetHiddenInGame` (`self.Cube`) false false))

(fn `OnRep_bIsSelected?`
  (if (`self.bIsSelected?`)
    (`MeshComponent.SetVectorParameterValueOnMaterials` (`self.Cube`) "None" (`KismetMathLibrary.Conv_LinearColorToVector` (struct :`R` 1.0 :`G` 0.5 :`A` 1.0)))
    (else
      (`MeshComponent.SetVectorParameterValueOnMaterials` (`self.Cube`) "None" (`KismetMathLibrary.Conv_LinearColorToVector` (struct :`R` 1.0 :`G` 0.5 :`A` 1.0))))))

(fn `OnTileInteract`
  (params (PlayerController :type "PlayerController Object Reference"))
  (set `self.InteractingPlayerController` PlayerController)
  (`self.SelectedPlayerController`
    (:`then`
      (if (== (`self.SelectedPlayerController`) (`self.InteractingPlayerController`))
        (set `self.bIsSelected?` false)))
    (:`else`
      (set `self.SelectedPlayerController` (`self.InteractingPlayerController`))
      (set `self.bIsSelected?` true))))

(fn `RemovePlayerSelection`
  (params (PlayerController :type "PlayerController Object Reference"))
  (set `self.bIsSelected?` false)
  (bind _asbp_ps_spawn_tile (cast `/Game/SpawnTile/Player/BP_PS_SpawnTile` (`Controller.PlayerState` PlayerController)))
  (`/Game/SpawnTile/Player/BP_PS_SpawnTile.SERVER_ActionSpawn` :`self` _asbp_ps_spawn_tile))

(fn `SetPlayerSelection`
  (params (PlayerController :type "PlayerController Object Reference"))
  (set `self.bIsSelected?` false)
  (bind _asbp_ps_spawn_tile (cast `/Game/SpawnTile/Player/BP_PS_SpawnTile` (`Controller.PlayerState` PlayerController)))
  (`/Game/SpawnTile/Player/BP_PS_SpawnTile.SERVER_ActionSpawn` _asbp_ps_spawn_tile null (`SceneComponent.GetRelativeTransform` (`self.Arrow`))))

(fn `ShowSpawnTile`
  (for _ (`PrimitiveComponent.GetOverlappingActors` (`self.Collision_Sphere`) "/Game/SpawnTile/Character/BP_Character_SpawnTile.BP_Character_SpawnTile_C")
    _)
  (`SceneComponent.SetHiddenInGame` (`self.Cube`) true false))

(fn `UserConstructionScript`)