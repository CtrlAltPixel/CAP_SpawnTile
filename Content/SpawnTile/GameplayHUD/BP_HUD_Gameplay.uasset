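; BP_HUD_Gameplay is the gameplay HUD Blueprint that creates the player's UI widgets and adds them to the viewport.
; BeginPlay creates WB_HUD, then runs init events for the match time and notification widgets.
; A separate event, not triggered in this file, shows the dead overlay.
; These three init events reuse valid cached widget references, and debug prints are gated by ShowDebug.
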(event `self.ReceiveBeginPlay`
  (`|ExecutionSequence`
    (:`then_0`
      (if (`self.bShowDebug?`)
        (`KismetSystemLibrary.PrintString` "BP_HUD_Gameplay - EVENT Begin Play" true true (struct :`G` 0.66 :`B` 1.0 :`A` 1.0) 3.0)))
    (:`then_1`
      (bind _returnvalue (`|CreateWidget` "/Game/SpawnTile/GameplayHUD/WB_HUD.WB_HUD_C" (`GameplayStatics.GetPlayerController` 0)))
      (set `self.As WB_HUD` _returnvalue)
      (`UserWidget.AddToViewport` (`self.As WB_HUD`) 0)
      (`self.EventHUDInitWBMatchTime`)
      (`self.EventHUDInitWBNotification`))))

(event `EventHUDInitWBDeadOverlay`
  (`|ExecutionSequence`
    (:`then_0`
      (if (`self.bShowDebug?`)
        (`KismetSystemLibrary.PrintString` "BP_HUD_Gameplay - EVENT HUD Init WB_DeadOverlay" true true (struct :`G` 0.66 :`B` 1.0 :`A` 1.0) 3.0)))
    (:`then_1`
      (`self.As WB_DeadOverlay`
        (:`then`
          _)
        (:`else`
          (bind _returnvalue (`|CreateWidget` "/Game/SpawnTile/GameplayHUD/Dead/WB_DeadOverlay.WB_DeadOverlay_C" (`GameplayStatics.GetPlayerController` 0)))
          (set `self.As WB_DeadOverlay` _returnvalue)))
      (`UserWidget.AddToViewport` (`self.As WB_DeadOverlay`) 0))))

(event `EventHUDInitWBNotification`
  (`|ExecutionSequence`
    (:`then_0`
      (if (`self.bShowDebug?`)
        (`KismetSystemLibrary.PrintString` "BP_HUD_Gameplay - EVENT HUD Init WB_Notification" true true (struct :`G` 0.66 :`B` 1.0 :`A` 1.0) 3.0)))
    (:`then_1`
      (`self.As WB_Notification`
        (:`then`
          _)
        (:`else`
          (bind _returnvalue (`|CreateWidget` "/Game/SpawnTile/GameplayHUD/Notification/WB_Notification.WB_Notification_C" (`GameplayStatics.GetPlayerController` 0)))
          (set `self.As WB_Notification` _returnvalue)))
      (`UserWidget.AddToViewport` (`self.As WB_Notification`) 0))))

(event `EventHUDInitWBMatchTime`
  (`|ExecutionSequence`
    (:`then_0`
      (if (`self.bShowDebug?`)
        (`KismetSystemLibrary.PrintString` "BP_HUD_Gameplay - EVENT HUD Init WB_MatchTime" true true (struct :`G` 0.66 :`B` 1.0 :`A` 1.0) 3.0)))
    (:`then_1`
      (`self.As WB_MatchTime`
        (:`then`
          _)
        (:`else`
          (bind _returnvalue (`|CreateWidget` "/Game/SpawnTile/GameplayHUD/MatchTime/WB_MatchTime.WB_MatchTime_C" (`GameplayStatics.GetPlayerController` 0)))
          (set `self.As WB_MatchTime` _returnvalue)))
      (`UserWidget.AddToViewport` (`self.As WB_MatchTime`) 0))))

(fn `InitCasts`
  (cast `/Game/SpawnTile/Blueprints/Player/Controller/BP_PC_Gameplay` (`GameplayStatics.GetPlayerController` 0)))

(fn `UserConstructionScript`)