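; BP_Actor_ActionEffect is an action effect actor in SpawnTile that provides activate and deactivate hooks but contains no effect logic of its own.
; EventActionEffectActivate calls the OnActionEffectStart dispatcher and EventActionEffectDeactivate calls OnActionEffectEnd.
; Both events and BeginPlay log through DebugMessage with the ShowDebug flag, all printing the same "EVENT Begin Play" text.
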(event `self.ReceiveBeginPlay`
  (`|ExecutionSequence`
    (:`then_0`
      (`/Game/SpawnTile/Gameplay/System/CommonFunctionLibrary.DebugMessage` "BP_Actor_ActionEffect - EVENT Begin Play" (`self.bShowDebug?`)))))

(event `EventActionEffectActivate`
  (`|ExecutionSequence`
    (:`then_0`
      (`/Game/SpawnTile/Gameplay/System/CommonFunctionLibrary.DebugMessage` "BP_Actor_ActionEffect - EVENT Begin Play" (`self.bShowDebug?`)))
    (:`then_1`
      (`self.OnActionEffectStart`))))

(event `EventActionEffectDeactivate`
  (`|ExecutionSequence`
    (:`then_0`
      (`/Game/SpawnTile/Gameplay/System/CommonFunctionLibrary.DebugMessage` "BP_Actor_ActionEffect - EVENT Begin Play" (`self.bShowDebug?`)))
    (:`then_1`
      (`self.OnActionEffectEnd`))))

(fn `UserConstructionScript`)