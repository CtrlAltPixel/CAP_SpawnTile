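; BP_AC_Interact is an actor component that sets up interaction collision and a hidden decal under its owner.
; On BeginPlay it gets the owner's interact capsule through a message call and sets it to overlap GameTraceChannel1.
; It then spawns a decal at the base of the owner's bounds, sized from their extent.
; A function toggles decal visibility; the dynamic material it creates is stored but never applied here.
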(event `self.ReceiveBeginPlay`
  (`|ExecutionSequence`
    (:`then_0`
      (`/Game/SpawnTile/Gameplay/System/CommonFunctionLibrary.DebugMessage` "BP AC Interact - EVENT Begin Play" (`self.bShowDebug`)))
    (:`then_1`
      (bind _capsulecollision (message `/Game/SpawnTile/Blueprints/Interact/Interface/BPI_Interact.GetInteractCapsule` (`self.GetOwner`)))
      (`PrimitiveComponent.SetCollisionResponseToChannel` _capsulecollision "ECC_GameTraceChannel1" "ECR_Overlap"))
    (:`then_2`
      (`self.EventDecalInit`))))

(event `EventDecalInit`
  (`|ExecutionSequence`
    (:`then_0`
      (`/Game/SpawnTile/Gameplay/System/CommonFunctionLibrary.DebugMessage` "BP Character Unit - EVENT Decal Init" (`self.bShowDebug`)))
    (:`then_1`
      (`self.AsDecalInteractComponent`
        (:`then`)
        (:`else`
          (bind _decalcomponent (`self.Func_SpawnDecalComponent`))
          (set `self.AsDecalInteractComponent` _decalcomponent)
          (bind _returnvalue (`KismetMaterialLibrary.CreateDynamicMaterialInstance` "/Game/SpawnTile/Blueprints/Interact/Material/MAT_Decal_Interact.MAT_Decal_Interact"))
          (set `self.AsMatDecalInteract` _returnvalue))))
    (:`then_2`
      (`self.Func_UpdateDecalVisibility` false))))

(fn `Func_SpawnDecalComponent`
  (returns (DecalComponent :type "DecalComponent Object Reference"))
  (bind _returnvalue (`self.GetOwner`))
  (bind (_origin _boxextent) (`Actor.GetActorBounds` _returnvalue false false))
  (`|ExecutionSequence`
    (:`then_0`
      (`/Game/SpawnTile/Gameplay/System/CommonFunctionLibrary.DebugMessage` "BP_AC_Team - FUNC Spawn Decal Component" (`self.bShowDebug`)))
    (:`then_1`
      (bind _returnvalue_2 (`GameplayStatics.SpawnDecalAttached` "/Game/SpawnTile/Blueprints/Interact/Material/MAT_Decal_Interact.MAT_Decal_Interact" (+ _boxextent 25.0) (`Actor.RootComponent` _returnvalue) "None" (- (`Actor.K2_GetActorLocation` _returnvalue) (`KismetMathLibrary.MakeVector` 0.0 0.0 (.z _boxextent))) (`KismetMathLibrary.Conv_VectorToRotator` (`Actor.GetActorUpVector` _returnvalue)) "KeepWorldPosition"))
      (return _returnvalue_2))))

(fn `Func_UpdateDecalVisibility`
  (params (bNewVisibility :type Boolean))
  (`|ExecutionSequence`
    (:`then_0`
      (`/Game/SpawnTile/Gameplay/System/CommonFunctionLibrary.DebugMessage` "BP_AC_Team - FUNC Update Decal Visibility" (`self.bShowDebug`)))
    (:`then_1`
      (bind _asdecalinteractcomponent (`self.AsDecalInteractComponent`)
        (:`then`
          (`SceneComponent.SetVisibility` _asdecalinteractcomponent bNewVisibility false))
        (:`else`)))))

(fn `GetInteractCapsule`
  (returns (CapsuleCollision :type "CapsuleComponent Object Reference"))
  (return null))