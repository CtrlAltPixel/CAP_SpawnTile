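; Tile actor variant that spawns a unit through the gameplay game mode as soon as a player state is added to it.
; On BeginPlay it caches BP_GM_Gameplay.
; Its player-state-add override runs the parent logic, then asks the game mode to spawn a unit at the tile's transform.
; The spawn always passes player controller 0, regardless of which player state was added.
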(event `self.ReceiveBeginPlay`
  (`parent.ReceiveBeginPlay`)
  (bind _asbp_gm_gameplay (cast `/Game/SpawnTile/Gameplay/System/GameMode/BP_GM_Gameplay` (`GameplayStatics.GetGameMode`)))
  (set `self.As_BP_GM_Gameplay` _asbp_gm_gameplay))

(event `self.EventTilePlayerStateAdd`
  (params (PlayerState :type "PlayerState Object Reference"))
  (`parent.EventTilePlayerStateAdd` PlayerState)
  (bind _as_bp_gm_gameplay (`self.As_BP_GM_Gameplay`)
    (:`then`
      (`/Game/SpawnTile/Gameplay/System/GameMode/BP_GM_Gameplay.EventGameModeUnitSpawn` _as_bp_gm_gameplay (`self.GetTransform`) (`GameplayStatics.GetPlayerController` 0)))
    (:`else`)))

(fn `UserConstructionScript`
  (`parent.UserConstructionScript`))