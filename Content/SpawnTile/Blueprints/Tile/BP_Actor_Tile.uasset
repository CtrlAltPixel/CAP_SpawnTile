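; BP_Actor_Tile is a replicated tile actor that a single player can select, colored to show who holds it.
; BeginPlay makes its collision box block a custom trace channel and disables collision on the visible cube mesh.
; The Add event claims a free tile or releases it for the same player, while Remove only releases.
; SelectedPlayerState's RepNotify tints the dynamic material as default, local owner or other player's selection.
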(event `self.ReceiveBeginPlay`
  (`|ExecutionSequence`
    (:`then_0`
      (if (`self.bShowDebug?`)
        (`KismetSystemLibrary.PrintString` "BP_Actor_Tile - EVENT BeginPlay" true true (struct :`G` 0.66 :`B` 1.0 :`A` 1.0) 3.0)))
    (:`then_1`
      (`PrimitiveComponent.SetCollisionResponseToChannel` (`self.Collision_Box`) "ECC_GameTraceChannel2" "ECR_Block")
      (`PrimitiveComponent.SetCollisionEnabled` (`self.StaticMesh_Cube`) "NoCollision")
      (`SceneComponent.SetVisibility` (`self.StaticMesh_Cube`) true false)
      (`self.SetReplicates` true))))

(event `EventTilePlayerStateAdd`
  (params (PlayerState :type "PlayerState Object Reference"))
  (`|ExecutionSequence`
    (:`then_0`
      (if (`self.bShowDebug?`)
        (`KismetSystemLibrary.PrintString` "BP_Actor_Tile - EVENT Player State Added" true true (struct :`G` 0.66 :`B` 1.0 :`A` 1.0) 3.0)))
    (:`then_1`
      (`/Engine/EditorBlueprintResources/StandardMacros.IsValid` PlayerState
        (:`Is Valid`
          (bind _selectedplayerstate (`self.SelectedPlayerState`)
            (:`then`
              (if (== _selectedplayerstate PlayerState)
                (bind _output_get (set `self.SelectedPlayerState` null))
                (`KismetSystemLibrary.PrintString` (`KismetSystemLibrary.GetDisplayName` _output_get))))
            (:`else`
              (bind _output_get_2 (set `self.SelectedPlayerState` PlayerState))
              (`KismetSystemLibrary.PrintString` (`KismetSystemLibrary.GetDisplayName` _output_get_2)))))))))

(event `EventTilePlayerStateRemove`
  (params (PlayerState :type "PlayerState Object Reference"))
  (`|ExecutionSequence`
    (:`then_0`
      (if (`self.bShowDebug?`)
        (`KismetSystemLibrary.PrintString` "BP_Actor_Tile - EVENT Player State Removed" true true (struct :`G` 0.66 :`B` 1.0 :`A` 1.0) 3.0)))
    (:`then_1`
      (`/Engine/EditorBlueprintResources/StandardMacros.IsValid` PlayerState
        (:`Is Valid`
          (bind _selectedplayerstate (`self.SelectedPlayerState`)
            (:`then`
              (if (== _selectedplayerstate PlayerState)
                (set `self.SelectedPlayerState` null)))
            (:`else`)))))))

(fn `OnRep_SelectedPlayerState`
  (bind _selectedplayerstate (`self.SelectedPlayerState`)
    (:`then`
      (if (== (`Controller.PlayerState` (`GameplayStatics.GetPlayerController` 0)) _selectedplayerstate)
        (`MaterialInstanceDynamic.SetVectorParameterValue` (`self.As DMI_Tile`) "Color" (`self.OwnerColor`))
        (else
          (`MaterialInstanceDynamic.SetVectorParameterValue` (`self.As DMI_Tile`) "Color" (`self.SelectedColor`)))))
    (:`else`
      (`MaterialInstanceDynamic.SetVectorParameterValue` (`self.As DMI_Tile`) "Color" (`self.DefaultColor`)))))

(fn `UserConstructionScript`
  (`|ExecutionSequence`
    (:`then_0`
      (if (`self.bShowDebug?`)
        (`KismetSystemLibrary.PrintString` "BP_Actor_Tile - EVENT Construct" true true (struct :`G` 0.66 :`B` 1.0 :`A` 1.0) 3.0)))
    (:`then_1`
      (bind _returnvalue (`PrimitiveComponent.CreateDynamicMaterialInstance` (`self.StaticMesh_Cube`) 0 "/Game/SpawnTile/Blueprints/Tile/Material/MAT_Tile.MAT_Tile" "None"))
      (set `self.As DMI_Tile` _returnvalue))))