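; BP_Actor_Tile_Turn is a tile actor whose cube mesh shows or hides with the gameplay turn phase.
; On BeginPlay it casts the game state to BP_GS_Gameplay, caches it and binds to its phase update event.
; The phase change handler shows the cube during Player Planning and hides it during Resolve Spells.
; A ShowDebug flag gates the debug prints.
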(event `self.ReceiveBeginPlay`
  (`parent.ReceiveBeginPlay`)
  (`|ExecutionSequence`
    (:`then_0`
      (if (`self.bShowDebug?`)
        (`KismetSystemLibrary.PrintString` "BP_Actor_Tile_Turn - EVENT Begin Play" true true (struct :`G` 0.66 :`B` 1.0 :`A` 1.0) 3.0)))
    (:`then_1`
      (bind _asbp_gs_gameplay (cast `/Game/SpawnTile/Gameplay/System/GameState/BP_GS_Gameplay` (`GameplayStatics.GetGameState`)))
      (bind _output_get (set `self.As BP GS Gameplay` _asbp_gs_gameplay))
      (add `/Game/SpawnTile/Gameplay/System/GameState/BP_GS_Gameplay.OnPhaseUpdate` _output_get (`|CreateDelegate` :!event `EventTileOnPhaseChange`)))))

(event `EventTileOnPhaseChange`
  (params (CurrentPhase :type "/Game/SpawnTile/Gameplay/System/Enum/E_Phase Enum" :default "NewEnumerator9"))
  (`|ExecutionSequence`
    (:`then_0`
      (if (`self.bShowDebug?`)
        (`KismetSystemLibrary.PrintString` "BP_Actor_Tile - EVENT Player State Added" true true (struct :`G` 0.66 :`B` 1.0 :`A` 1.0) 3.0)))
    (:`then_1`
      (switch `/Game/SpawnTile/Gameplay/System/Enum/E_Phase` CurrentPhase
        (:`NewEnumerator0`
          (`SceneComponent.SetVisibility` (`self.StaticMesh_Cube`) true false))
        (:`NewEnumerator7`
          (`SceneComponent.SetVisibility` (`self.StaticMesh_Cube`) false false))))))

(fn `UserConstructionScript`
  (`parent.UserConstructionScript`))