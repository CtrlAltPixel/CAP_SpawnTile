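; Turn-based spawn tile actor that toggles its cube mesh's visibility with the game phase.
; On BeginPlay it binds to the phase update event on BP_GS_Gameplay.
; On each change, if the first player controller has no valid character unit, it shows the cube only during PlayerPlanning and hides it otherwise.
; With a valid unit, visibility is left unchanged.
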(event `self.ReceiveBeginPlay`
  (`parent.ReceiveBeginPlay`)
  (`self.EventTileBindToPhaseChange`))

(event `EventTileBindToPhaseChange`
  (`|ExecutionSequence`
    (:`then_0`
      (`/Game/SpawnTile/Gameplay/System/CommonFunctionLibrary.DebugMessage` "BP_Actor_Tile_Turnbase - EVENT Bind to phase change" (`self.bShowDebug`)))
    (:`then_1`
      (bind _asbp_gs_gameplay (cast `/Game/SpawnTile/Gameplay/System/GameState/BP_GS_Gameplay` (`GameplayStatics.GetGameState`)))
      (add `/Game/SpawnTile/Gameplay/System/GameState/BP_GS_Gameplay.OnPhaseUpdate` _asbp_gs_gameplay (`|CreateDelegate` :!event `EventTileOnPhaseChange`)))))

(event `EventTileOnPhaseChange`
  (params (CurrentPhase :type "/Game/SpawnTile/Gameplay/System/Enum/E_Phase Enum" :default "NewEnumerator9"))
  (`|ExecutionSequence`
    (:`then_0`
      (`/Game/SpawnTile/Gameplay/System/CommonFunctionLibrary.DebugMessage` "BP_Actor_Tile_Turnbase - EVENT Bind to phase change" (`self.bShowDebug`)))
    (:`then_1`
      (bind _asbp_pc_gameplay (cast `/Game/SpawnTile/Gameplay/Player/Controller/BP_PC_Gameplay` (`GameplayStatics.GetPlayerController` 0)))
      (`/Game/SpawnTile/Gameplay/Player/Controller/BP_PC_Gameplay.As BP Character Unit_` _asbp_pc_gameplay
        (:`then`)
        (:`else`
          (`self.Func_TileUpdateMeshVisibility` CurrentPhase))))))

(fn `Func_TileUpdateMeshVisibility`
  (params (Phase :type "/Game/SpawnTile/Gameplay/System/Enum/E_Phase Enum" :default "NewEnumerator9"))
  (`SceneComponent.SetVisibility` (`self.StaticMesh_Cube`) (select `/Game/SpawnTile/Gameplay/System/Enum/E_Phase` Phase :`NewEnumerator0` true) false))

(fn `UserConstructionScript`
  (`parent.UserConstructionScript`))