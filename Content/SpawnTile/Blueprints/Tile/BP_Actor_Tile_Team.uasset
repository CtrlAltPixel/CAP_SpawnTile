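; BP_Actor_Tile_Team is a tile actor variant colored by the team it belongs to.
; Its construction script runs the parent's, prints an optional debug message, then maps the Team value to a blue or red DefaultColor.
; That color is written to the Color parameter of the tile's dynamic material instance.
; BeginPlay only calls the parent, and Tick is disabled.
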(event `self.ReceiveBeginPlay`
  (`parent.ReceiveBeginPlay`))

(fn `UserConstructionScript`
  (`parent.UserConstructionScript`)
  (`|ExecutionSequence`
    (:`then_0`
      (if (`self.bShowDebug?`)
        (`KismetSystemLibrary.PrintString` "BP_Actor_Tile_Team - EVENT Construct" true true (struct :`G` 0.66 :`B` 1.0 :`A` 1.0) 3.0)))
    (:`then_1`
      (switch `/Game/SpawnTile/Blueprints/Team/Enum/E_Team` (`self.Team`)
        (:`NewEnumerator1`
          (set `self.DefaultColor` (struct :`B` 1.0 :`A` 1.0)))
        (:`NewEnumerator3`
          (set `self.DefaultColor` (struct :`R` 1.0 :`A` 1.0)))))
    (:`then_2`
      (`MaterialInstanceDynamic.SetVectorParameterValue` (`self.As DMI_Tile`) "Color" (`self.DefaultColor`)))))