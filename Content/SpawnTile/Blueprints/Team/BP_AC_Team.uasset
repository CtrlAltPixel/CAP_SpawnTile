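; Team actor component that stores its owner's team and is meant to tint a team decal to match.
; UpdateTeam stores the new value and calls UpdateDecalColor, which picks a Blue, Red, Neutral or Spectator color for a valid DecalTeam; GetTeam returns the stored team.
; Decal spawning and attachment are disconnected, so BeginPlay and the InitDecal event only print debug messages and nothing here creates the decal.
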(event `self.ReceiveBeginPlay`
  (`|ExecutionSequence`
    (:`then_0`
      (if (`self.bShowDebug?`)
        (`KismetSystemLibrary.PrintString` "BP_AC_Team - EVENT Begin Play" true true (struct :`G` 0.66 :`B` 1.0 :`A` 1.0) 3.0)))
    (:`then_1`
      (if true
        _))))

(event `EventACTeamInitDecal`
  (`|ExecutionSequence`
    (:`then_0`
      (if (`self.bShowDebug?`)
        (`KismetSystemLibrary.PrintString` "BP_AC_Team - EVENT InitDecal" true true (struct :`G` 0.66 :`B` 1.0 :`A` 1.0) 3.0)))))

(fn `GetTeam`
  (returns (Team :type "/Game/SpawnTile/Blueprints/Team/Enum/E_Team Enum"))
  (return (`self.Team`)))

(fn `UpdateDecalColor`
  (params (Team :type "/Game/SpawnTile/Blueprints/Team/Enum/E_Team Enum" :default "NewEnumerator0"))
  (`|ExecutionSequence`
    (:`then_0`
      (if (`self.bShowDebug?`)
        (`KismetSystemLibrary.PrintString` "BP_AC_Team - FUNC UpdateDecalColor" true true (struct :`G` 0.66 :`B` 1.0 :`A` 1.0) 3.0)))
    (:`then_1`
      (bind _decal_team (`self.Decal_Team`)
        (:`then`
          (`DecalComponent.SetDecalColor` _decal_team (select `/Game/SpawnTile/Blueprints/Team/Enum/E_Team` Team :`NewEnumerator1` (`self.BlueTeamColor`) :`NewEnumerator2` (`self.NeutralTeamColor`) :`NewEnumerator3` (`self.RedTeamColor`) :`NewEnumerator4` (`self.SpectatorTeamColor`))))
        (:`else`)))))

(fn `UpdateTeam`
  (params (Team :type "/Game/SpawnTile/Blueprints/Team/Enum/E_Team Enum" :default "NewEnumerator0"))
  (set `self.Team` Team)
  (`self.UpdateDecalColor` "NewEnumerator0"))