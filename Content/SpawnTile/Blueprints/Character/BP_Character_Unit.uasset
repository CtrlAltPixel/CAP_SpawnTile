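; Character Blueprint for a SpawnTile unit, handling its initial hidden state, animation montages and death registration.
; On BeginPlay it sets the capsule to block a custom trace channel, then hides itself and disables collision.
; MULTIPlayAnimMontage plays and tracks the current montage, firing begin and end callbacks, with completion, blend-out and interruption sharing the end path.
; Death registration notifies BP_GM_Gameplay, casting and caching the game mode if needed.
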(event `self.ReceiveBeginPlay`
  (`|ExecutionSequence`
    (:`then_0`
      (`/Game/SpawnTile/Blueprints/System/CommonFunctionLibrary.DebugMessage` "BP Character Unit - EVENT BeginPlay" (`self.bShowDebug?`)))
    (:`then_1`
      (`PrimitiveComponent.SetCollisionResponseToChannel` (`self.CapsuleComponent`) "ECC_GameTraceChannel1" "ECR_Block")
      (`self.SetActorHidden` true))))

(event `MULTIPlayAnimMontage`
  (params (AnimMontage :type "AnimMontage Object Reference"))
  (`|ExecutionSequence`
    (:`then_0`
      (if (`self.bShowDebug?`)
        (`KismetSystemLibrary.PrintString` "BP Character Unit - EVENT AnimMontage" true true (struct :`G` 0.66 :`B` 1.0 :`A` 1.0) 3.0)))
    (:`then_1`
      (bind _output_get (set `self.AsCurrentAnimMontage` AnimMontage))
      (`|PlayMontage` (`self.Mesh`) _output_get
        (:`then`
          (`self.OnAimMontageBegin`))
        (:`OnCompleted`
          (set `self.AsCurrentAnimMontage` null :!label _label)
          (`self.OnAnimMontageEnd`))
        (:`OnBlendOut`
          (goto _label))
        (:`OnInterrupted`
          (goto _label))))))

(event `EventUnitRegisterDeath`
  (`|ExecutionSequence`
    (:`then_0`
      (if (`self.bShowDebug?`)
        (`KismetSystemLibrary.PrintString` "BP Character Unit - EVENT Destroy" true true (struct :`G` 0.66 :`B` 1.0 :`A` 1.0) 3.0)))
    (:`then_1`
      (`self.As BP GM Spawn Tiler`
        (:`then`
          _)
        (:`else`
          (bind _asbp_gm_gameplay (cast `/Game/SpawnTile/Blueprints/System/Modes/BP_GM_Gameplay` (`GameplayStatics.GetGameMode`)))
          (set `self.As BP GM Spawn Tiler` _asbp_gm_gameplay)))
      (`/Game/SpawnTile/Blueprints/System/Modes/BP_GM_Gameplay.EventGameModeCharacterDied` (`self.As BP GM Spawn Tiler`) self))))

(fn `SetActorHidden`
  (params (bNewHidden :type Boolean))
  (`self.SetActorHiddenInGame` bNewHidden)
  (`self.SetActorEnableCollision` (not bNewHidden)))

(fn `UserConstructionScript`)