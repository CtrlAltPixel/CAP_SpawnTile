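; AI controller for NPCs that holds the current action state for spawn, movement, dash, preparation, spell, combat and death.
; Each update event stores the action it receives in the matching variable, with no logic here that acts on those values.
; A ShowDebug flag gates on-screen prints, which are labeled BP_AIController_Gameplay, and the death event's print reads "Update Combat".
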(event `self.ReceiveBeginPlay`
  (`|ExecutionSequence`
    (:`then_0`
      (if (`self.bShowDebug?`)
        (`KismetSystemLibrary.PrintString` "BP_AIController_Gameplay - EVENT Begin Play" true true (struct :`G` 0.66 :`B` 1.0 :`A` 1.0) 3.0)))))

(event `EventAIControllerUpdateSpell`
  (params (PlanningAction :type "/Game/SpawnTile/Blueprints/Action/BP_AC_Action Class Reference"))
  (`|ExecutionSequence`
    (:`then_0`
      (if (`self.bShowDebug?`)
        (`KismetSystemLibrary.PrintString` "BP_AIController_Gameplay - EVENT Update Spell" true true (struct :`G` 0.66 :`B` 1.0 :`A` 1.0) 3.0)))
    (:`then_1`
      (set `self.SpellAction` PlanningAction))))

(event `EventAIControllerUpdatePreperation`
  (params (PlanningAction :type "/Game/SpawnTile/Blueprints/Action/BP_AC_Action Class Reference"))
  (`|ExecutionSequence`
    (:`then_0`
      (if (`self.bShowDebug?`)
        (`KismetSystemLibrary.PrintString` "BP_AIController_Gameplay - EVENT Update Planning" true true (struct :`G` 0.66 :`B` 1.0 :`A` 1.0) 3.0)))
    (:`then_1`
      (set `self.PreperationAction` PlanningAction))))

(event `EventAIControllerUpdateDash`
  (params (DashAction :type "/Game/SpawnTile/Blueprints/Action/BP_AC_Action Class Reference"))
  (`|ExecutionSequence`
    (:`then_0`
      (if (`self.bShowDebug?`)
        (`KismetSystemLibrary.PrintString` "BP_AIController_Gameplay - EVENT Update Dash" true true (struct :`G` 0.66 :`B` 1.0 :`A` 1.0) 3.0)))
    (:`then_1`
      (set `self.DashAction` DashAction))))

(event `EentAIControllerUpdateCombat`
  (params (CombatAction :type "/Game/SpawnTile/Blueprints/Action/BP_AC_Action Class Reference"))
  (`|ExecutionSequence`
    (:`then_0`
      (if (`self.bShowDebug?`)
        (`KismetSystemLibrary.PrintString` "BP_AIController_Gameplay - EVENT Update Combat" true true (struct :`G` 0.66 :`B` 1.0 :`A` 1.0) 3.0)))
    (:`then_1`
      (set `self.CombatAction` CombatAction))))

(event `EventAIControllerUpdateDeath`
  (params (DeathAction :type "/Game/SpawnTile/Blueprints/Action/BP_AC_Action Class Reference"))
  (`|ExecutionSequence`
    (:`then_0`
      (if (`self.bShowDebug?`)
        (`KismetSystemLibrary.PrintString` "BP_AIController_Gameplay - EVENT Update Combat" true true (struct :`G` 0.66 :`B` 1.0 :`A` 1.0) 3.0)))
    (:`then_1`
      (set `self.DeathAction` DeathAction))))

(event `EventAIControllerUpdateMovement`
  (params (MovementAction :type "/Game/SpawnTile/Blueprints/Action/BP_AC_Action Class Reference"))
  (`|ExecutionSequence`
    (:`then_0`
      (if (`self.bShowDebug?`)
        (`KismetSystemLibrary.PrintString` "BP_AIController_Gameplay - EVENT Update Movement" true true (struct :`G` 0.66 :`B` 1.0 :`A` 1.0) 3.0)))
    (:`then_1`
      (set `self.MovementAction` MovementAction))))

(event `EventAIControllerUpdateSpawn`
  (params (SpawnAction :type "/Game/SpawnTile/Blueprints/Action/BP_AC_Action Class Reference"))
  (`|ExecutionSequence`
    (:`then_0`
      (if (`self.bShowDebug?`)
        (`KismetSystemLibrary.PrintString` "BP_AIController_Gameplay - EVENT Update Spawn" true true (struct :`G` 0.66 :`B` 1.0 :`A` 1.0) 3.0)))
    (:`then_1`
      (set `self.SpawnAction` SpawnAction))))

(fn `UserConstructionScript`)