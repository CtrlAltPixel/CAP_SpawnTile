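; Action component for unit actors that runs a list of action effects, each represented by an actor class.
; On BeginPlay, if the owner is a BP_Character_Unit tagged "Unit", it spawns the first effect, binds to its end dispatcher and signals action start.
; EventActionEnd removes the head entry and calls itself until the list empties, spawning no further effects, then signals action end.
; The add and remove effect functions are empty stubs.
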(event `self.ReceiveBeginPlay`
  (bind _returnvalue (`self.GetOwner`))
  (`|ExecutionSequence`
    (:`then_0`
      (if (`self.bShowDebug?`)
        (`KismetSystemLibrary.PrintString` "BP_AC_Actions - EVENT Begin Play")))
    (:`then_1`
      (if (`Actor.ActorHasTag` _returnvalue "Unit")
        (bind _asbp_character_unit (cast `/Game/SpawnTile/Blueprints/Character/BP_Character_Unit` _returnvalue))
        (set `self.As BP Character Unit` _asbp_character_unit)
        (`self.EventActionStart`)
        (`self.OnActionStart`)))))

(event `EventActionStart`
  (bind _returnvalue (`|SpawnActorFromClass` (`|GetArrayItem` (`self.Action Effects`)) (`KismetMathLibrary.MakeTransform` (0.0 0.0 0.0)) "Undefined" "MultiplyWithRoot" null null))
  (bind _output_get (set `self.As BP_Actor_ActionEffect` _returnvalue))
  (add `/Game/SpawnTile/Blueprints/Action/BP_Actor_ActionEffect.OnActionEffectEnd` _output_get (`|CreateDelegate` :!event `EventActionEnd`)))

(event `EventActionEnd`
  (`KismetArrayLibrary.Array_Remove` (`self.Action Effects`))
  (if (`KismetArrayLibrary.Array_IsEmpty` (`self.Action Effects`))
    (`self.OnActionEnd`)
    (else
      (`self.EventActionEnd`))))

(fn `Func_AddActionEffect`)

(fn `Func_GetActionEffect`
  (returns (`Action Effects` :type "Array of /Game/SpawnTile/Blueprints/Action/BP_Actor_ActionEffect Class Reference"))
  (return (`self.Action Effects`)))

(fn `Func_RemoveActionEfffect`)