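; Gameplay game mode that tracks joined player controllers and spawns their units from each controller's loadout message.
; On a controller swap it copies the loadout to the new controller and spawns that unit under its ownership.
; A spawn event, acting only on authority, places the player's loadout unit at an action effect's location and rotation.
; Death handling is a stub, and an AI unit spawn sits unconnected.
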(event `self.ReceiveBeginPlay`
  (add `self.OnPlayerDied` (`|CreateDelegate` :!event `EventGameModeCharacterDied`)))

(event `self.K2_PostLogin`
  (params (NewPlayer :type "PlayerController Object Reference"))
  (`KismetArrayLibrary.Array_Add` (`self.AllPlayerControllers`) NewPlayer))

(event `self.K2_OnSwapPlayerControllers`
  (params (OldPC :type "PlayerController Object Reference") (NewPC :type "PlayerController Object Reference"))
  (bind _loadout (message `/Game/SpawnTile/Loadout/BPI_Loadouts.GetLoadout` OldPC))
  (message `/Game/SpawnTile/Loadout/BPI_Loadouts.SetLoadout` NewPC _loadout)
  (`|SpawnActorFromClass` (`.Unit_2_DBBEAB05485632D68729B9BA3FFCEAD3` (break `/Game/SpawnTile/Loadout/FLoadout` _loadout)) (`KismetMathLibrary.MakeTransform` (0.0 0.0 0.0)) "Undefined" "MultiplyWithRoot" NewPC 1 null))

(event `self.K2_OnLogout`
  (params (ExitingController :type "Controller Object Reference"))
  (bind _asplayer_controller (cast `PlayerController` ExitingController))
  (`KismetArrayLibrary.Array_RemoveItem` (`self.AllPlayerControllers`) _asplayer_controller))

(event `EventGameModeSpawnPlayerUnit`
  (params (PlayerState :type "PlayerState Object Reference") (ActionEffect :type "/Game/SpawnTile/Blueprints/Action/BP_Actor_ActionEffect Object Reference"))
  (bind _returnvalue (`PlayerState.GetPlayerController` PlayerState))
  (`/Engine/EditorBlueprintResources/StandardMacros.IsValid` PlayerState
    (:`Is Valid`
      (`/Engine/EditorBlueprintResources/ActorMacros.Switch Has Authority`
        (:`Authority`
          (bind _loadout (message `/Game/SpawnTile/Loadout/BPI_Loadouts.GetLoadout` _returnvalue))
          (`|SpawnActorFromClass` (break `/Game/SpawnTile/Loadout/FLoadout` _loadout) (`KismetMathLibrary.MakeTransform` (`self.K2_GetActorLocation` ActionEffect) (`self.K2_GetActorRotation` ActionEffect)) "Undefined" "MultiplyWithRoot" _returnvalue 0 null))))))

(event `EventGameModeCharacterDied` :!signature `self.OnPlayerDied`
  (params (Character :type "Character Object Reference"))
  (`|ExecutionSequence`
    (:`then_0`
      (if (`self.bShowDebug?`)
        _))
    (:`then_1`
      (cast `/Game/SpawnTile/Blueprints/Character/Player/BP_Character_Player` Character))))

(fn `UserConstructionScript`)