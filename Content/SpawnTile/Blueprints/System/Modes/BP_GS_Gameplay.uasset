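; Game State for SpawnTile's turn-based match, driving match, turn, phase and action events from authority until a kill or turn limit.
; Each turn opens with timed player planning, followed by resolve phases from spells to respawn.
; Resolve phases queue units with a matching AI controller action, focus all cameras on each and add that action as a component.
; Queue sorting, input toggling, settings and phase widget are stubs, and phase advancing never calls PhaseStart here.
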(event `self.ReceiveBeginPlay`
  (`|ExecutionSequence`
    (:`then_0`
      (if (`self.bShowDebug?`)
        (`KismetSystemLibrary.PrintString` "BP_GS_Gameplay - EVENT BeginPlay" true true (struct :`G` 0.66 :`B` 1.0 :`A` 1.0) 3.0)))
    (:`then_1`
      (`/Engine/EditorBlueprintResources/ActorMacros.Switch Has Authority`
        (:`Authority`
          (`KismetSystemLibrary.Delay` 3.0)
          (`self.EventGameStateMatchStart`))))))

(event `EventGameStateMatchStart`
  (`|ExecutionSequence`
    (:`then_0`
      (if (`self.bShowDebug?`)
        (`KismetSystemLibrary.PrintString` "BP_GS_Gameplay - EVENT StartMatch" true true (struct :`G` 0.66 :`B` 1.0 :`A` 1.0) 3.0)))
    (:`then_1`
      (`self.Func_UpdateMatchSetting`)
      (`self.Func_StartMatchTimer`)
      (`self.EventGameStateTurnStart`))))

(event `EventGameStateUpdateMatchTimer`
  (`|ExecutionSequence`
    (:`then_0`
      (if (`self.bShowDebug?`)
        (`KismetSystemLibrary.PrintString` "BP_GS_Gameplay - EVENT Update Match Timer" true true (struct :`G` 0.66 :`B` 1.0 :`A` 1.0) 3.0)))
    (:`then_1`
      (set `self.MatchTime` (+ (`self.MatchTime`) 1)))))

(event `EventGameStateMatchEnd`
  (`|ExecutionSequence`
    (:`then_0`
      (if (`self.bShowDebug?`)
        (`KismetSystemLibrary.PrintString` "BP_GS_Gameplay - EVENT EndMatch" true true (struct :`G` 0.66 :`B` 1.0 :`A` 1.0) 3.0)))
    (:`then_1`
      (`KismetSystemLibrary.K2_ClearAndInvalidateTimerHandle` (`self.MatchTimer`)))))

(event `EventGameStateTurnStart`
  (`|ExecutionSequence`
    (:`then_0`
      (if (`self.bShowDebug?`)
        (`KismetSystemLibrary.PrintString` "BP_GS_Gameplay - EVENT Turn Start" true true (struct :`G` 0.66 :`B` 1.0 :`A` 1.0) 3.0)))
    (:`then_1`
      (`self.Func_UpdateTurnCount`)
      (`self.Func_FocusOwnUnit`)
      (`self.Func_EnableInput`)
      (set `self.Phase` "NewEnumerator0")
      (`self.EventGameStatePhaseStart`))))

(event `EventGameStateTurnEnd`
  (`|ExecutionSequence`
    (:`then_0`
      (if (`self.bShowDebug?`)
        (`KismetSystemLibrary.PrintString` "BP_GS_Gameplay - EVENT Turn End" true true (struct :`G` 0.66 :`B` 1.0 :`A` 1.0) 3.0)))
    (:`then_1`
      (bind _bsuccess_ (`self.Func_MaxKills`))
      (if _bsuccess_
        (`self.EventGameStateMatchEnd`)
        (else
          (bind _bsuccess__2 (`self.Func_MaxTurns`))
          (if _bsuccess__2
            (`self.EventGameStateMatchEnd`)
            (else
              (`self.EventGameStateTurnStart`))))))))

(event `EventGameStatePhaseStart`
  (`|ExecutionSequence`
    (:`then_0`
      (if (`self.bShowDebug?`)
        (`KismetSystemLibrary.PrintString` "BP_GS_Gameplay - EVENT PhaseStart" true true (struct :`G` 0.66 :`B` 1.0 :`A` 1.0) 3.0)))
    (:`then_1`
      (switch `/Game/SpawnTile/Blueprints/System/Enum/E_Phase` (`self.Phase`)
        (:`NewEnumerator0`
          (`self.Func_FocusOwnUnit`)
          (`self.Func_EnableInput`)
          (`self.Func_StartPlanningTimer`))
        (:`NewEnumerator7`
          (`self.Func_ShowPhaseWidget` (`self.Phase`) :!label _label)
          (bind _unitstoaction (`self.Func_CreateUnitQue`))
          (set `self.UnitQue` _unitstoaction)
          (`self.Func_SortUnitQue` (`self.UnitQue`))
          (`self.EventGameStateActionStart`))
        (:`NewEnumerator6`
          (goto _label))
        (:`NewEnumerator3`
          (goto _label))
        (:`NewEnumerator4`
          (goto _label))
        (:`NewEnumerator2`
          (goto _label))
        (:`NewEnumerator5`
          (goto _label))
        (:`NewEnumerator1`
          (goto _label))))))

(event `EventGameStateUpdateReadyTimer`
  (bind _readytime (`self.ReadyTime`))
  (`|ExecutionSequence`
    (:`then_0`
      (if (`self.bShowDebug?`)
        (`KismetSystemLibrary.PrintString` "BP_GS_Gameplay - EVENT Update Ready Timer" true true (struct :`G` 0.66 :`B` 1.0 :`A` 1.0) 3.0)))
    (:`then_1`
      (if (> _readytime 0)
        (set `self.ReadyTime` (- _readytime 1))))))

(event `EventGameStatePhaseEnd`
  (`|ExecutionSequence`
    (:`then_0`
      (if (`self.bShowDebug?`)
        (`KismetSystemLibrary.PrintString` "BP_GS_Gameplay - EVENT PhaseEnd" true true (struct :`G` 0.66 :`B` 1.0 :`A` 1.0) 3.0)))
    (:`then_1`
      (switch `/Game/SpawnTile/Blueprints/System/Enum/E_Phase` (`self.Phase`)
        (:`NewEnumerator0`
          (`self.Func_DisableInput`)
          (`self.Func_UpdatePhase`))
        (:`NewEnumerator7`
          (`self.Func_UpdatePhase` :!label _label_2))
        (:`NewEnumerator6`
          (goto _label_2))
        (:`NewEnumerator3`
          (goto _label_2))
        (:`NewEnumerator4`
          (goto _label_2))
        (:`NewEnumerator2`
          (goto _label_2))
        (:`NewEnumerator5`
          (goto _label_2))
        (:`NewEnumerator1`
          (`self.EventGameStateTurnEnd`))))))

(event `EventGameStateActionStart`
  (`|ExecutionSequence`
    (:`then_0`
      (if (`self.bShowDebug?`)
        (`KismetSystemLibrary.PrintString` "BP_GS_Gameplay - EVENT ActionStart" true true (struct :`G` 0.66 :`B` 1.0 :`A` 1.0) 3.0)))
    (:`then_1`
      (bind _output_get (set `self.CurrentUnit` (`|GetArrayItem` (`self.UnitQue`))))
      (bind _asbp_aicontroller_spawn_tile (cast `/Game/SpawnTile/Blueprints/Character/AI/BP_AIController_SpawnTile` (`Pawn.GetController` _output_get)))
      (set `self.CurrentAIController` _asbp_aicontroller_spawn_tile)
      (`self.Func_AllFocusCamera` (`self.CurrentUnit`))
      (switch `/Game/SpawnTile/Blueprints/System/Enum/E_Phase` (`self.Phase`)
        (:`NewEnumerator7`
          (bind _currentaicontroller (`self.CurrentAIController`)
            (:`then`
              (`|AddComponentByClass` (`self.CurrentUnit`) (`/Game/SpawnTile/Blueprints/Character/AI/BP_AIController_SpawnTile.SpellAction` _currentaicontroller)))
            (:`else`)))
        (:`NewEnumerator6`
          (bind _currentaicontroller_2 (`self.CurrentAIController`)
            (:`then`
              (`|AddComponentByClass` (`self.CurrentUnit`) (`/Game/SpawnTile/Blueprints/Character/AI/BP_AIController_SpawnTile.PreperationAction` _currentaicontroller_2)))
            (:`else`)))
        (:`NewEnumerator3`
          (bind _currentaicontroller_3 (`self.CurrentAIController`)
            (:`then`
              (`|AddComponentByClass` (`self.CurrentUnit`) (`/Game/SpawnTile/Blueprints/Character/AI/BP_AIController_SpawnTile.DashAction` _currentaicontroller_3)))
            (:`else`)))
        (:`NewEnumerator4`
          (bind _currentaicontroller_4 (`self.CurrentAIController`)
            (:`then`
              (`|AddComponentByClass` (`self.CurrentUnit`) (`/Game/SpawnTile/Blueprints/Character/AI/BP_AIController_SpawnTile.CombatAction` _currentaicontroller_4)))
            (:`else`)))
        (:`NewEnumerator2`
          (bind _currentaicontroller_5 (`self.CurrentAIController`)
            (:`then`
              (`|AddComponentByClass` (`self.CurrentUnit`) (`/Game/SpawnTile/Blueprints/Character/AI/BP_AIController_SpawnTile.DeathAction` _currentaicontroller_5)))
            (:`else`)))
        (:`NewEnumerator5`
          (bind _currentaicontroller_6 (`self.CurrentAIController`)
            (:`then`
              (`|AddComponentByClass` (`self.CurrentUnit`) (`/Game/SpawnTile/Blueprints/Character/AI/BP_AIController_SpawnTile.MovementAction` _currentaicontroller_6)))
            (:`else`)))
        (:`NewEnumerator1`
          (bind _currentaicontroller_7 (`self.CurrentAIController`)
            (:`then`
              (`|AddComponentByClass` (`self.CurrentUnit`) (`/Game/SpawnTile/Blueprints/Character/AI/BP_AIController_SpawnTile.SpawnAction` _currentaicontroller_7)))
            (:`else`)))))))

(event `EventGameStateActionEnd`
  (`|ExecutionSequence`
    (:`then_0`
      (if (`self.bShowDebug?`)
        (`KismetSystemLibrary.PrintString` "BP_GS_Gameplay - EVENT ActionEnd" true true (struct :`G` 0.66 :`B` 1.0 :`A` 1.0) 3.0)))
    (:`then_1`
      (`KismetArrayLibrary.Array_RemoveItem` (`self.UnitQue`) (`self.CurrentUnit`))
      (set `self.CurrentUnit` null)
      (if (`KismetArrayLibrary.Array_IsEmpty` (`self.UnitQue`))
        (`self.EventGameStatePhaseEnd`)
        (else
          (`self.EventGameStateActionStart`))))))

(fn `Func_AllFocusCamera`
  (params (ActorToFocus :type "Actor Object Reference"))
  (locals (Local_PlayerController :type "/Game/SpawnTile/Blueprints/Player/Controller/BP_PC_Gameplay Object Reference"))
  (for _array_element (`self.PlayerArray`)
    (bind _asbp_pc_gameplay (cast `/Game/SpawnTile/Blueprints/Player/Controller/BP_PC_Gameplay` (`PlayerState.GetPlayerController` _array_element)))
    (bind _output_get (set `local.Local_PlayerController` _asbp_pc_gameplay))
    (bind _as_bp_pawn_camera (`/Game/SpawnTile/Blueprints/Player/Controller/BP_PC_Gameplay.As BP Pawn Camera` _output_get)
      (:`then`
        (`/Game/SpawnTile/Blueprints/Player/Camera/BP_Pawn_Camera.CameraFocus` _as_bp_pawn_camera (`local.ActorToFocus`)))
      (:`else`)))
  (return))

(fn `Func_AllPlayersReady`
  (returns (`bAllReady?` :type Boolean))
  (locals (Local_AllReady :type Boolean))
  (for _array_element (`self.PlayerArray`)
    (cast `/Game/SpawnTile/Blueprints/Player/State/BP_PS_Gameplay` _array_element))
  (return (`local.Local_AllReady`)))

(fn `Func_CreateUnitQue`
  (returns (UnitsToAction :type "Array of Pawn Object Reference"))
  (locals (Local_AiController :type "/Game/SpawnTile/Blueprints/Character/AI/BP_AIController_SpawnTile Object Reference") (Local_Unit :type "/Game/SpawnTile/Blueprints/Character/BP_Character_Unit Object Reference") (Local_UnitQue :type "Array of Pawn Object Reference"))
  (`KismetArrayLibrary.Array_Clear` (`local.Local_UnitQue`))
  (bind _outactors (`GameplayStatics.GetAllActorsOfClass` "/Game/SpawnTile/Blueprints/Character/BP_Character_Unit.BP_Character_Unit_C"))
  (for _array_element _outactors
    (bind _output_get (set `local.Local_Unit` _array_element))
    (bind _asbp_aicontroller_spawn_tile (cast `/Game/SpawnTile/Blueprints/Character/AI/BP_AIController_SpawnTile` (`AIBlueprintHelperLibrary.GetAIController` _output_get)))
    (set `local.Local_AiController` _asbp_aicontroller_spawn_tile)
    (switch `/Game/SpawnTile/Blueprints/System/Enum/E_Phase` (`self.Phase`)
      (:`NewEnumerator7`
        (`/Game/SpawnTile/Blueprints/Character/AI/BP_AIController_SpawnTile.SpellAction` (`local.Local_AiController`)
          (:`then`
            (`KismetArrayLibrary.Array_Add` (`local.Local_UnitQue`) (`local.Local_Unit`)))
          (:`else`)))
      (:`NewEnumerator6`
        (`/Game/SpawnTile/Blueprints/Character/AI/BP_AIController_SpawnTile.PreperationAction` (`local.Local_AiController`)
          (:`then`
            (`KismetArrayLibrary.Array_Add` (`local.Local_UnitQue`) (`local.Local_Unit`)))
          (:`else`)))
      (:`NewEnumerator3`
        (`/Game/SpawnTile/Blueprints/Character/AI/BP_AIController_SpawnTile.DashAction` (`local.Local_AiController`)
          (:`then`
            (`KismetArrayLibrary.Array_Add` (`local.Local_UnitQue`) (`local.Local_Unit`)))
          (:`else`)))
      (:`NewEnumerator4`
        (`/Game/SpawnTile/Blueprints/Character/AI/BP_AIController_SpawnTile.CombatAction` (`local.Local_AiController`)
          (:`then`
            (`KismetArrayLibrary.Array_Add` (`local.Local_UnitQue`) (`local.Local_Unit`)))
          (:`else`)))
      (:`NewEnumerator2`
        (`/Game/SpawnTile/Blueprints/Character/AI/BP_AIController_SpawnTile.DeathAction` (`local.Local_AiController`)
          (:`then`
            (`KismetArrayLibrary.Array_Add` (`local.Local_UnitQue`) (`local.Local_Unit`)))
          (:`else`)))
      (:`NewEnumerator5`
        (`/Game/SpawnTile/Blueprints/Character/AI/BP_AIController_SpawnTile.MovementAction` (`local.Local_AiController`)
          (:`then`
            (`KismetArrayLibrary.Array_Add` (`local.Local_UnitQue`) (`local.Local_Unit`)))
          (:`else`)))
      (:`NewEnumerator1`
        (`/Game/SpawnTile/Blueprints/Character/AI/BP_AIController_SpawnTile.SpawnAction` (`local.Local_AiController`)
          (:`then`
            (`KismetArrayLibrary.Array_Add` (`local.Local_UnitQue`) (`local.Local_Unit`)))
          (:`else`)))))
  (return (`local.Local_UnitQue`)))

(fn `Func_DisableInput`
  (for _ (`self.PlayerArray`)
    _))

(fn `Func_EnableInput`
  (for _ (`self.PlayerArray`)
    _))

(fn `Func_FocusOwnUnit`
  (locals (Local_PlayerController :type "/Game/SpawnTile/Blueprints/Player/Controller/BP_PC_Gameplay Object Reference"))
  (for _array_element (`self.PlayerArray`)
    (bind _asbp_pc_gameplay (cast `/Game/SpawnTile/Blueprints/Player/Controller/BP_PC_Gameplay` (`PlayerState.GetPlayerController` _array_element)))
    (bind _output_get (set `local.Local_PlayerController` _asbp_pc_gameplay))
    (bind _as_bp_character_unit (`/Game/SpawnTile/Blueprints/Player/Controller/BP_PC_Gameplay.As BP Character Unit` _output_get)
      (:`then`
        (bind _as_bp_pawn_camera (`/Game/SpawnTile/Blueprints/Player/Controller/BP_PC_Gameplay.As BP Pawn Camera` _output_get)
          (:`then`
            (`/Game/SpawnTile/Blueprints/Player/Camera/BP_Pawn_Camera.CameraFocus` _as_bp_pawn_camera _as_bp_character_unit))
          (:`else`)))
      (:`else`)))
  (return))

(fn `Func_MaxKills`
  (returns (`bSuccess?` :type Boolean))
  (return (or (> (`self.BlueKillCount`) (`self.Setting_MaxKills`)) (> (`self.RedKillCount`) (`self.Setting_MaxKills`)))))

(fn `Func_MaxTurns`
  (returns (`bSuccess?` :type Boolean))
  (return (>= (`self.TurnCount`) (`self.Setting_MaxTurns`))))

(fn `Func_ShowPhaseWidget`
  (params (Phase :type "/Game/SpawnTile/Blueprints/System/Enum/E_Phase Enum" :default "NewEnumerator9")))

(fn `Func_SortUnitQue`
  (params (QueToSort :type "Array of Pawn Object Reference"))
  (returns (OrderedUnitQue :type "Array of Pawn Object Reference"))
  (locals (Local_PlayerStates :type "Array of PlayerState Object Reference") (Local_AiController :type "/Game/SpawnTile/Blueprints/Character/AI/BP_AIController_SpawnTile Object Reference")))

(fn `Func_StartMatchTimer`
  (bind _returnvalue (`KismetSystemLibrary.K2_SetTimer` null "EventGameStateUpdateMatchTimer" 1.0 true))
  (set `self.MatchTimer` _returnvalue))

(fn `Func_StartPlanningTimer`
  (bind _returnvalue (`KismetSystemLibrary.K2_SetTimer` null "EventGameStateUpdateReadyTimer" 0.1 true))
  (set `self.ReadyTimer` _returnvalue))

(fn `Func_UpdateMatchSetting`)

(fn `Func_UpdatePhase`
  (bind _result (`/Engine/EditorBlueprintResources/StandardMacros.IncrementInt` (`KismetMathLibrary.Conv_ByteToInt` (`self.Phase`)))
    (:`  `
      (set `self.Phase` (cast `/Game/SpawnTile/Blueprints/System/Enum/E_Phase` (`KismetMathLibrary.Conv_IntToByte` (mod _result (enumcount `/Game/SpawnTile/Blueprints/System/Enum/E_Phase`))))))))

(fn `Func_UpdateTurnCount`
  (set `self.TurnCount` (+ (`self.TurnCount`) 1)))

(fn `OnRep_Phase`
  (`self.OnPhaseEnd` (`self.Phase`)))

(fn `UserConstructionScript`)