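; BP_Character_Unit is a character Blueprint for units in the SpawnTile game.
; On BeginPlay it sets the SpawnTile AI controller class and makes the capsule block a custom trace channel.
; MULTIPlayAnimMontage, named as a multicast, plays a montage on the mesh, tracks it as current and signals begin and end, treating blend-out and interruption as end.
; On destruction it reports the death to the spawn-tile game mode reference, if valid.
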(event `self.ReceiveBeginPlay`
  (`|ExecutionSequence`
    (:`then_0`
      (if (`self.bShowDebug?`)
        (`KismetSystemLibrary.PrintString` "BP Character Unit - EVENT BeginPlay" true true (struct :`G` 0.66 :`B` 1.0 :`A` 1.0) 3.0)))
    (:`then_1`
      (set `self.AIControllerClass` "/Game/SpawnTile/Character/AI/BP_AIController_SpawnTile.BP_AIController_SpawnTile_C")
      (`PrimitiveComponent.SetCollisionResponseToChannel` (`self.CapsuleComponent`) "ECC_GameTraceChannel1" "ECR_Block"))))

(event `MULTIPlayAnimMontage`
  (params (AnimMontage :type "AnimMontage Object Reference"))
  (`|ExecutionSequence`
    (:`then_0`
      (if (`self.bShowDebug?`)
        _))
    (:`then_1`
      (bind _output_get (set `self.AsCurrentAnimMontage` AnimMontage))
      (`|PlayMontage` (`self.Mesh`) _output_get
        (:`then`
          (`self.OnAimMontageBegin`))
        (:`OnCompleted`
          (set `self.AsCurrentAnimMontage` null :!label _label)
          (`self.OnAnimMontageEnd`))
        (:`OnBlendOut`
          (goto _label))
        (:`OnInterrupted`
          (goto _label))))))

(event `self.ReceiveDestroyed`
  (`|ExecutionSequence`
    (:`then_0`
      (if (`self.bShowDebug?`)
        _))
    (:`then_1`
      (bind _as_bp_gm_spawn_tiler (`self.As BP GM Spawn Tiler`)
        (:`then`
          (`/Game/SpawnTile/Modes/BP_GM_Gameplay.EventCharacterDied` _as_bp_gm_spawn_tiler self)
          (`KismetSystemLibrary.PrintString` "Destroy Character"))
        (:`else`)))))

(fn `UserConstructionScript`)