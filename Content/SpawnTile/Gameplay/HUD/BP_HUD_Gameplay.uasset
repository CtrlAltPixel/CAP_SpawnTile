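; BP_HUD_Gameplay is the gameplay HUD that creates and manages the player's on-screen widgets.
; On BeginPlay it adds the main HUD, then runs init events for the dead overlay, notification and debug widgets, reusing valid instances.
; The unit update event hides the dead overlay when given a valid character unit and shows it otherwise.
; Weapon init and update events are stubs that only log debug messages.
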(event `self.ReceiveBeginPlay`
  (`|ExecutionSequence`
    (:`then_0`
      (`/Game/SpawnTile/Gameplay/System/CommonFunctionLibrary.DebugMessage` "BP_HUD_Gameplay - EVENT Begin Play" (`self.bShowDebug?`)))
    (:`then_1`
      (bind _returnvalue (`|CreateWidget` "/Game/SpawnTile/Gameplay/HUD/WB_HUD.WB_HUD_C" (`GameplayStatics.GetPlayerController` 0)))
      (set `self.AsWB_HUD` _returnvalue)
      (`UserWidget.AddToViewport` (`self.AsWB_HUD`) 0))
    (:`then_2`
      (`self.EventHUDInitWBDeadOverlay`)
      (`self.EventHUDInitWBNotification`)
      (`self.EventHUDWBPDebugInit`))))

(event `EventHUDWBPDebugInit`
  (`|ExecutionSequence`
    (:`then_0`
      (`/Game/SpawnTile/Gameplay/System/CommonFunctionLibrary.DebugMessage` "BP_HUD_Gameplay - EVENT HUD Init WB_DeadOverlay" (`self.bShowDebug?`)))
    (:`then_1`
      (`self.AsWBP_Debug`
        (:`then`
          _)
        (:`else`
          (bind _returnvalue (`|CreateWidget` "/Game/SpawnTile/Gameplay/HUD/Debug/WBP_Debug.WBP_Debug_C" (`GameplayStatics.GetPlayerController` 0)))
          (set `self.AsWBP_Debug` _returnvalue)))
      (`UserWidget.AddToViewport` (`self.AsWBP_Debug`) 0))))

(event `EventHUDInitWBDeadOverlay`
  (bind _aswb_deadoverlay (`self.AsWB_DeadOverlay`))
  (`|ExecutionSequence`
    (:`then_0`
      (`/Game/SpawnTile/Gameplay/System/CommonFunctionLibrary.DebugMessage` "BP_HUD_Gameplay - EVENT HUD Init WB_DeadOverlay" (`self.bShowDebug?`)))
    (:`then_1`
      (`self.AsWB_DeadOverlay`
        (:`then`
          _)
        (:`else`
          (bind _returnvalue (`|CreateWidget` "/Game/SpawnTile/Gameplay/HUD/Dead/WBP_DeadOverlay.WBP_DeadOverlay_C" (`GameplayStatics.GetPlayerController` 0)))
          (set `self.AsWB_DeadOverlay` _returnvalue)))
      (`UserWidget.AddToViewport` _aswb_deadoverlay 0)
      (`/Game/SpawnTile/Gameplay/HUD/Dead/WBP_DeadOverlay.EventWBPDeadOverlayUpdateVisibility` _aswb_deadoverlay true))))

(event `EventHUDInitWBNotification`
  (`|ExecutionSequence`
    (:`then_0`
      (`/Game/SpawnTile/Gameplay/System/CommonFunctionLibrary.DebugMessage` "BP_HUD_Gameplay - EVENT HUD Init WB_Notification" (`self.bShowDebug?`)))
    (:`then_1`
      (`self.AsWB_Notification`
        (:`then`
          _)
        (:`else`
          (bind _returnvalue (`|CreateWidget` "/Game/SpawnTile/Gameplay/HUD/Notification/WBP_Notification.WBP_Notification_C" (`GameplayStatics.GetPlayerController` 0)))
          (set `self.AsWB_Notification` _returnvalue)))
      (`UserWidget.AddToViewport` (`self.AsWB_Notification`) 0))))

(event `EventHUDInitWBPWeapon`
  (`|ExecutionSequence`
    (:`then_0`
      (`/Game/SpawnTile/Gameplay/System/CommonFunctionLibrary.DebugMessage` "BP_HUD_Gameplay - EVENT HUD Init WB_Notification" (`self.bShowDebug?`)))))

(event `EventWBPHUDUpdateUnit`
  (params (AsBP_Character_Unit :type "/Game/SpawnTile/Gameplay/Unit/BP_Character_Unit Object Reference"))
  (`|ExecutionSequence`
    (:`then_0`
      (`/Game/SpawnTile/Gameplay/System/CommonFunctionLibrary.DebugMessage` "BP_HUD_Gameplay - EVENT HUD Update Unit On Owning Client" (`self.bShowDebug?`)))
    (:`then_1`
      (`/Engine/EditorBlueprintResources/StandardMacros.IsValid` AsBP_Character_Unit
        (:`Is Valid`
          (bind _aswb_deadoverlay (`self.AsWB_DeadOverlay`)
            (:`then`
              (`/Game/SpawnTile/Gameplay/HUD/Dead/WBP_DeadOverlay.EventWBPDeadOverlayUpdateVisibility` _aswb_deadoverlay false))
            (:`else`)))
        (:`Is Not Valid`
          (bind _aswb_deadoverlay_2 (`self.AsWB_DeadOverlay`)
            (:`then`
              (`/Game/SpawnTile/Gameplay/HUD/Dead/WBP_DeadOverlay.EventWBPDeadOverlayUpdateVisibility` _aswb_deadoverlay_2 true))
            (:`else`)))))))

(event `EventHUDWeaponUpdate`
  (params (Loadout :type "/Game/SpawnTile/Blueprints/Loadout/F_Loadout Structure"))
  (`|ExecutionSequence`
    (:`then_0`
      (`/Game/SpawnTile/Gameplay/System/CommonFunctionLibrary.DebugMessage` "BP_HUD_Gameplay - EVENT HUD Update Weapon UI" (`self.bShowDebug?`)))))

(fn `InitCasts`
  (cast `/Game/SpawnTile/Gameplay/Player/Controller/BP_PC_Gameplay` (`GameplayStatics.GetPlayerController` 0)))

(fn `UserConstructionScript`)