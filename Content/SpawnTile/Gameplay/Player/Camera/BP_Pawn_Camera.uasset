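; BP_Pawn_Camera is a player camera pawn that exposes events for moving, rotating, zooming and focusing the view.
; Move feeds two input axes into movement input along the pawn's right and forward vectors, while focus snaps the pawn to a valid actor's location without sweeping.
; Rotate and zoom only print debug messages, which ShowDebug gates throughout, and InitCasts is empty.
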(event `self.ReceiveBeginPlay`
  (`|ExecutionSequence`
    (:`then_0`
      (if (`self.bShowDebug?`)
        (`KismetSystemLibrary.PrintString` "BP_Pawn_Camera - EVENT BeginPlay" true true (struct :`G` 0.66 :`B` 1.0 :`A` 1.0) 3.0)))))

(event `self.ReceivePossessed`
  (params (NewController :type "Controller Object Reference"))
  (`|ExecutionSequence`
    (:`then_0`
      (if (`self.bShowDebug?`)
        (`KismetSystemLibrary.PrintString` "BP_Pawn_Camera - EVENT Possessed" true true (struct :`G` 0.66 :`B` 1.0 :`A` 1.0) 3.0)))))

(event `CameraMove`
  (params (InputAxisX :type "Float (double-precision)") (InputAxisY :type "Float (double-precision)"))
  (`|ExecutionSequence`
    (:`then_0`
      (if (`self.bShowDebug?`)
        (`KismetSystemLibrary.PrintString` "BP_Pawn_Camera - EVENT Camera Move" true true (struct :`G` 0.66 :`B` 1.0 :`A` 1.0) 3.0)))
    (:`then_1`
      (`self.AddMovementInput` (`self.GetActorRightVector`) InputAxisX)
      (`self.AddMovementInput` (`self.GetActorForwardVector`) InputAxisY))))

(event `EventCameraRotate`
  (params (InputAxis :type Boolean))
  (`|ExecutionSequence`
    (:`then_0`
      (if (`self.bShowDebug?`)
        (`KismetSystemLibrary.PrintString` "BP_Pawn_Camera - EVENT Camera Rotate" true true (struct :`G` 0.66 :`B` 1.0 :`A` 1.0) 3.0)))))

(event `EventCameraZoom`
  (params (InputAxis :type Boolean))
  (`|ExecutionSequence`
    (:`then_0`
      (if (`self.bShowDebug?`)
        (`KismetSystemLibrary.PrintString` "BP_Pawn_Camera - EVENT Camera Zoom" true true (struct :`G` 0.66 :`B` 1.0 :`A` 1.0) 3.0)))))

(event `CameraFocus`
  (params (ActorToFocus :type "Actor Object Reference"))
  (`|ExecutionSequence`
    (:`then_0`
      (if (`self.bShowDebug?`)
        (`KismetSystemLibrary.PrintString` "BP_Pawn_Camera - EVENT Camera Focus" true true (struct :`G` 0.66 :`B` 1.0 :`A` 1.0) 3.0)))
    (:`then_1`
      (`/Engine/EditorBlueprintResources/StandardMacros.IsValid` ActorToFocus
        (:`Is Valid`
          (`self.K2_SetActorLocation` self (`self.K2_GetActorLocation` ActorToFocus) false false))))))

(fn `InitCasts`)

(fn `UserConstructionScript`)