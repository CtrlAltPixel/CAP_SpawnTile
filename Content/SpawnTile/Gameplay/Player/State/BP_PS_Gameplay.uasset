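; BP_PS_Gameplay is the gameplay player state Blueprint that stores a player's IsReady and IsDead flags.
; Two custom events each write their incoming value to the matching flag, with debug messages indicating they are meant to run on the server.
; BeginPlay and both update events print debug messages when ShowDebug is enabled, while Tick and the construction script are empty.
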(event `self.ReceiveBeginPlay`
  (`|ExecutionSequence`
    (:`then_0`
      (if (`self.bShowDebug?`)
        (`KismetSystemLibrary.PrintString` "BP_PS_Gameplay - Event Begin Play" true true (struct :`G` 0.66 :`B` 1.0 :`A` 1.0) 3.0)))))

(event `EventPlayerStateUpdateIsReady?`
  (params (`bIsReady?` :type Boolean))
  (`|ExecutionSequence`
    (:`then_0`
      (if (`self.bShowDebug?`)
        (`KismetSystemLibrary.PrintString` "BP_PS_Gameplay - Event Update Player Ready On Server" true true (struct :`G` 0.66 :`B` 1.0 :`A` 1.0) 3.0)))
    (:`then_1`
      (set `self.bIsReady?` `bIsReady?`))))

(event `EventPlayerStateUpdateIsDead?`
  (params (`bIsDead?` :type Boolean))
  (`|ExecutionSequence`
    (:`then_0`
      (if (`self.bShowDebug?`)
        (`KismetSystemLibrary.PrintString` "BP_PS_Gameplay - Event Set Unit Dead on SERVER" true true (struct :`G` 0.66 :`B` 1.0 :`A` 1.0) 3.0)))
    (:`then_1`
      (set `self.bIsDead?` `bIsDead?`))))

(fn `UserConstructionScript`)