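; Gameplay player controller that sets up camera, HUD and tile input for the local player in a phase-based game.
; Enhanced Input contexts drive camera movement, actor interaction with drag and focus, and tile picking through cursor traces.
; Tile picks add or remove the PlayerState through Local/Server event pairs, and unit replication updates the HUD.
; Chosen actions route by phase to the unit AI controller; debug keys force GameState phases.
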(event Custom|DEBUGPlanningPhase
  (bind _asbp_gs_gameplay (Utilities|Casting|CastToBP_GS_Gameplay (Game|GetGameState)))
  (Default|EventGameStatePhaseUpdate _asbp_gs_gameplay "NewEnumerator0"))

(event Custom|DEBUGStartPhase
  (bind _asbp_gs_gameplay (Utilities|Casting|CastToBP_GS_Gameplay (Game|GetGameState)))
  (Default|EventGameStatePhaseStart _asbp_gs_gameplay))

(event Custom|DEBUGSpellPhase
  (bind _asbp_gs_gameplay (Utilities|Casting|CastToBP_GS_Gameplay (Game|GetGameState)))
  (Default|EventGameStatePhaseUpdate _asbp_gs_gameplay "NewEnumerator7"))

(event Custom|DEBUGDashPhase
  (bind _asbp_gs_gameplay (Utilities|Casting|CastToBP_GS_Gameplay (Game|GetGameState)))
  (Default|EventGameStatePhaseUpdate _asbp_gs_gameplay "NewEnumerator3"))

(event Custom|DEBUGPreperationPhase
  (bind _asbp_gs_gameplay (Utilities|Casting|CastToBP_GS_Gameplay (Game|GetGameState)))
  (Default|EventGameStatePhaseUpdate _asbp_gs_gameplay "NewEnumerator6"))

(event Custom|DEBUGCombatPhase
  (bind _asbp_gs_gameplay (Utilities|Casting|CastToBP_GS_Gameplay (Game|GetGameState)))
  (Default|EventGameStatePhaseUpdate _asbp_gs_gameplay "NewEnumerator4"))

(event Custom|DEBUGMovementPhase
  (bind _asbp_gs_gameplay (Utilities|Casting|CastToBP_GS_Gameplay (Game|GetGameState)))
  (Default|EventGameStatePhaseUpdate _asbp_gs_gameplay "NewEnumerator5"))

(event Custom|DEBUGSpawnPhase
  (bind _asbp_gs_gameplay (Utilities|Casting|CastToBP_GS_Gameplay (Game|GetGameState)))
  (Default|EventGameStatePhaseUpdate _asbp_gs_gameplay "NewEnumerator1"))

(event EventBeginPlay
  (if (Pawn|IsLocalPlayerController)
    (Utilities|FlowControl|Sequence
      (:then_0
        (if (Variables|Debug|GetbShowDebug?)
          (Development|PrintString "BP_PC_Gameplay - EVENT BeginPlay" true true "(R=0.000000,G=0.660000,B=1.000000,A=1.000000)" 3.0)))
      (:then_1
        (CallFunction|EventPlayerControllerInitCamera)
        (CallFunction|EventPlayerControllerInitHUD)
        (Variables|Default|SetbShowMouseCursor true)
        (Variables|Default|SetbEnableClickEvents true)
        (Variables|Default|SetbEnableMouseOverEvents true)
        (CallFunction|EventPlayerControllerInitTile)))))

(event Input|KeyboardEvents|DebugKey5
  (params (Key :type Key%20Structure :default "None") (ActionValue :type Input%20Action%20Value%20Structure))
  (:Pressed
    (CallFunction|DEBUGCombatPhase)))

(event Input|KeyboardEvents|DebugKey6
  (params (Key :type Key%20Structure :default "None") (ActionValue :type Input%20Action%20Value%20Structure))
  (:Pressed
    (CallFunction|DEBUGMovementPhase)))

(event Input|KeyboardEvents|DebugKey1
  (params (Key :type Key%20Structure :default "None") (ActionValue :type Input%20Action%20Value%20Structure))
  (:Pressed
    (CallFunction|DEBUGPlanningPhase)))

(event Input|KeyboardEvents|DebugKey2
  (params (Key :type Key%20Structure :default "None") (ActionValue :type Input%20Action%20Value%20Structure))
  (:Pressed
    (CallFunction|DEBUGSpellPhase)))

(event Input|KeyboardEvents|DebugKey3
  (params (Key :type Key%20Structure :default "None") (ActionValue :type Input%20Action%20Value%20Structure))
  (:Pressed
    (CallFunction|DEBUGPreperationPhase)))

(event Input|KeyboardEvents|DebugKey4
  (params (Key :type Key%20Structure :default "None") (ActionValue :type Input%20Action%20Value%20Structure))
  (:Pressed
    (CallFunction|DEBUGDashPhase)))

(event Input|KeyboardEvents|DebugKey7
  (params (Key :type Key%20Structure :default "None") (ActionValue :type Input%20Action%20Value%20Structure))
  (:Pressed
    (CallFunction|DEBUGSpawnPhase)))

(event Input|KeyboardEvents|DebugKey9
  (params (Key :type Key%20Structure :default "None") (ActionValue :type Input%20Action%20Value%20Structure))
  (:Pressed
    (CallFunction|DEBUGStartPhase)))

(event Custom|EventPlayerControllerInitCamera
  (bind _returnvalue (PlayerController|LocalPlayerSubsystems|GetEnhancedInputLocalPlayerSubsystem))
  (Utilities|FlowControl|Sequence
    (:then_0
      (if (Variables|Debug|GetbShowDebug?)
        (Development|PrintString "BP_PC_Gameplay - EVENT Init Camera" true true "(R=0.000000,G=0.660000,B=1.000000,A=1.000000)" 3.0)))
    (:then_1
      (Utilities|IsValid _returnvalue
        (:Is%20Valid
          (Input|AddMappingContext _returnvalue "/Game/SpawnTile/Gameplay/Player/Input/IMC_Camera.IMC_Camera" 0 "(bIgnoreAllPressedKeysUntilRelease=True,bForceImmediately=False,bNotifyUserSettings=False)")
          (Variables|Reference|GetAs%20BP%20Pawn%20Camera
            (:then
              (Actor|DestroyActor (Variables|Reference|GetAs%20BP%20Pawn%20Camera)))
            (:else
              _))
          (bind _asbp_pawn_camera (Utilities|Casting|CastToBP_Pawn_Camera (Pawn|GetControlledPawn))
            (:then
              (Variables|Reference|SetAs%20BP%20Pawn%20Camera _asbp_pawn_camera))
            (:CastFailed
              (if (Variables|Debug|GetbShowDebug?)
                (Development|PrintString "BP_PC_Gameplay - EVENT Init Camera FAILED to cast to BP_Pawn_Camera" true true "(R=0.000000,G=0.660000,B=1.000000,A=1.000000)" 3.0)))))
        (:Is%20Not%20Valid
          (if (Variables|Debug|GetbShowDebug?)
            (Development|PrintString "BP_PC_Gameplay - EVENT Init Camera INVALID Enhanced Input Subsytem" true true "(R=0.000000,G=0.660000,B=1.000000,A=1.000000)" 3.0)))))))

(event Input|EnhancedActionEvents|EnhancedInputActionIA_Camera_Move
  (params (ActionValue :type Vector%202D%20Structure) (ElapsedSeconds :type Float%20%28double-precision%29) (TriggeredSeconds :type Float%20%28double-precision%29) (InputAction :type Input%20Action%20Object%20Reference :default "/Game/SpawnTile/Gameplay/Player/Input/Actions/Camera/IA_Camera_Move.IA_Camera_Move"))
  (bind _as_bp_pawn_camera (Variables|Reference|GetAs%20BP%20Pawn%20Camera)
    (:then
      (Default|CameraMove _as_bp_pawn_camera (.x ActionValue) (.y ActionValue)))
    (:else)))

(event Custom|EventPlayerControllerInitInteract
  (bind _returnvalue (PlayerController|LocalPlayerSubsystems|GetEnhancedInputLocalPlayerSubsystem))
  (Utilities|FlowControl|Sequence
    (:then_0
      (if (Variables|Debug|GetbShowDebug?)
        (Development|PrintString "BP_PC_Gameplay - EVENT Init Interact" true true "(R=0.000000,G=0.660000,B=1.000000,A=1.000000)" 3.0)))
    (:then_1
      (Utilities|IsValid _returnvalue
        (:Is%20Valid
          (Input|AddMappingContext _returnvalue "/Game/SpawnTile/Gameplay/Player/Input/IMC_Interact.IMC_Interact" 0 "(bIgnoreAllPressedKeysUntilRelease=True,bForceImmediately=False,bNotifyUserSettings=False)")
          (Variables|Default|SetCurrentClickTraceChannel "ECC_GameTraceChannel1"))))))

(event Input|EnhancedActionEvents|EnhancedInputActionIA_Interact_Primary
  (params (ActionValue :type Boolean) (ElapsedSeconds :type Float%20%28double-precision%29) (TriggeredSeconds :type Float%20%28double-precision%29) (InputAction :type Input%20Action%20Object%20Reference :default "/Game/SpawnTile/Gameplay/Player/Input/Actions/Interact/IA_Interact_Primary.IA_Interact_Primary"))
  (bind (_hit _hitactor) (CallFunction|GetActorUnderCursorbyChannel "TraceTypeQuery3"))
  (bind _returnvalue (PlayerController|LocalPlayerSubsystems|GetEnhancedInputLocalPlayerSubsystem))
  (bind _returnvalue_2 (PlayerController|LocalPlayerSubsystems|GetEnhancedInputLocalPlayerSubsystem))
  (:Started
    (Utilities|FlowControl|Sequence
      (:then_0
        (if (Variables|Debug|GetbShowDebug?)
          (Development|PrintString "BP_PC_Gameplay - IA_INTERACT_PRIMARY" true true "(R=0.000000,G=0.660000,B=1.000000,A=1.000000)" 3.0)))
      (:then_1
        (if _hit
          (Variables|Default|GetAs%20BP_Interact_Actor
            (:then
              (Class|BPIInteract|EndInteract(Message) (Variables|Default|GetAs%20BP_Interact_Actor))
              (Variables|Default|SetAs%20BP_Interact_Actor 0)
              (bind _output_get (Variables|Default|SetAs%20BP_Interact_Actor _hitactor))
              (Class|BPIInteract|StartInteract(Message) _output_get))
            (:else
              (bind _output_get_2 (Variables|Default|SetAs%20BP_Interact_Actor _hitactor))
              (Class|BPIInteract|StartInteract(Message) _output_get_2)))
          (else
            (Utilities|IsValid _returnvalue_2
              (:Is%20Valid
                (Input|RemoveMappingContext _returnvalue_2 "/Game/SpawnTile/Gameplay/Player/Input/IMC_Interact.IMC_Interact" "(bIgnoreAllPressedKeysUntilRelease=True,bForceImmediately=False,bNotifyUserSettings=False)")
                (Input|AddMappingContext _returnvalue_2 "/Game/SpawnTile/Gameplay/Player/Input/IMC_Drag.IMC_Drag" 0 "(bIgnoreAllPressedKeysUntilRelease=True,bForceImmediately=False,bNotifyUserSettings=False)"))))))))
  (:Completed
    (Utilities|IsValid _returnvalue
      (:Is%20Valid
        (Input|RemoveMappingContext _returnvalue "/Game/SpawnTile/Gameplay/Player/Input/IMC_Drag.IMC_Drag" "(bIgnoreAllPressedKeysUntilRelease=True,bForceImmediately=False,bNotifyUserSettings=False)")
        (Input|AddMappingContext _returnvalue "/Game/SpawnTile/Gameplay/Player/Input/IMC_Interact.IMC_Interact" 0 "(bIgnoreAllPressedKeysUntilRelease=True,bForceImmediately=False,bNotifyUserSettings=False)")))))

(event Input|EnhancedActionEvents|EnhancedInputActionIA_Interact_Secondary
  (params (ActionValue :type Boolean) (ElapsedSeconds :type Float%20%28double-precision%29) (TriggeredSeconds :type Float%20%28double-precision%29) (InputAction :type Input%20Action%20Object%20Reference :default "/Game/SpawnTile/Gameplay/Player/Input/Actions/Interact/IA_Interact_Secondary.IA_Interact_Secondary"))
  (:Started
    (Utilities|FlowControl|Sequence
      (:then_0
        (if (Variables|Debug|GetbShowDebug?)
          (Development|PrintString "BP_PC_Gameplay - IA_INTERACT_SECONDARY" true true "(R=0.000000,G=0.660000,B=1.000000,A=1.000000)" 3.0)))
      (:then_1
        (bind _as_bp_interact_actor (Variables|Default|GetAs%20BP_Interact_Actor)
          (:then
            (Class|BPIInteract|EndInteract(Message) _as_bp_interact_actor)
            (Variables|Default|SetAs%20BP_Interact_Actor 0))
          (:else))))))

(event Input|EnhancedActionEvents|EnhancedInputActionIA_Interact_Focus
  (params (ActionValue :type Boolean) (ElapsedSeconds :type Float%20%28double-precision%29) (TriggeredSeconds :type Float%20%28double-precision%29) (InputAction :type Input%20Action%20Object%20Reference :default "/Game/SpawnTile/Gameplay/Player/Input/Actions/Interact/IA_Interact_Focus.IA_Interact_Focus"))
  (:Completed
    (Utilities|FlowControl|Sequence
      (:then_0
        (if (Variables|Debug|GetbShowDebug?)
          (Development|PrintString "BP_PC_Gameplay - IA_FOCUS" true true "(R=0.000000,G=0.660000,B=1.000000,A=1.000000)" 3.0)))
      (:then_1
        (bind _as_bp_pawn_camera (Variables|Reference|GetAs%20BP%20Pawn%20Camera)
          (:then
            (Default|CameraFocus _as_bp_pawn_camera (Variables|Default|GetAs%20BP_Interact_Actor)))
          (:else))))))

(event Custom|EventPlayerControllerUpdateUnit
  (params (Unit :type BP%20Character%20Unit%20Object%20Reference))
  (Variables|Default|SetAs%20BP%20Character%20Unit_ Unit))

(event Custom|EventPlayerControllerInitTile
  (bind _returnvalue (PlayerController|LocalPlayerSubsystems|GetEnhancedInputLocalPlayerSubsystem))
  (Utilities|FlowControl|Sequence
    (:then_0
      (if (Variables|Debug|GetbShowDebug?)
        (Development|PrintString "BP_PC_Gameplay - EVENT Init Tile" true true "(R=0.000000,G=0.660000,B=1.000000,A=1.000000)" 3.0)))
    (:then_1
      (Utilities|IsValid _returnvalue
        (:Is%20Valid
          (Input|AddMappingContext _returnvalue "/Game/SpawnTile/Gameplay/Player/Input/IMC_Tile.IMC_Tile" 0 "(bIgnoreAllPressedKeysUntilRelease=True,bForceImmediately=False,bNotifyUserSettings=False)")
          (Input|RemoveMappingContext _returnvalue "/Game/SpawnTile/Gameplay/Player/Input/IMC_Interact.IMC_Interact" "(bIgnoreAllPressedKeysUntilRelease=True,bForceImmediately=False,bNotifyUserSettings=False)")
          (Variables|Default|SetCurrentClickTraceChannel "ECC_GameTraceChannel2"))))))

(event Custom|EventTileUpdateVisibility
  (bind _asbp_gs_gameplay (Utilities|Casting|CastToBP_GS_Gameplay (Game|GetGameState)))
  (Variables|Default|GetAs%20BP%20Character%20Unit_
    (:then)
    (:else
      (bind _outactors (Actor|GetAllActorsOfClass "/Game/SpawnTile/Blueprints/Tile/BP_Actor_Tile.BP_Actor_Tile_C"))
      (for _array_element _outactors
        (Rendering|SetVisibility (Variables|/Game/SpawnTile/Blueprints/Tile/BP_Actor_Tile.BP_Actor_Tile_C|GetStaticMesh_Cube _array_element) (Utilities|Select :Index (Variables|/Game/SpawnTile/Gameplay/System/GameState/BP_GS_Gameplay.BP_GS_Gameplay_C|GetPhase _asbp_gs_gameplay) :NewEnumerator9 false :NewEnumerator0 true :NewEnumerator7 false :NewEnumerator6 false :NewEnumerator3 false :NewEnumerator4 false :NewEnumerator2 false :NewEnumerator5 false :NewEnumerator1 false) false)))))

(event Custom|EventPlayerControllerAddPlayerStateServer
  (params (Tile :type BP%20Actor%20Tile%20Object%20Reference) (PlayerState :type Player%20State%20Object%20Reference))
  (Utilities|IsValid Tile
    (:Is%20Valid
      (bind _output_get (Variables|Reference|SetAs%20BP%20Actor%20Tile Tile))
      (Default|EventTilePlayerStateAdd _output_get PlayerState))))

(event Custom|EventPlayerControllerRemovePlayerStateServer
  (params (PlayerState :type Player%20State%20Object%20Reference))
  (Utilities|FlowControl|Sequence
    (:then_0
      (if (Variables|Debug|GetbShowDebug?)
        (Development|PrintString "BP_PC_Gameplay - EVENT Remove PlayerState On Server" true true "(R=0.000000,G=0.660000,B=1.000000,A=1.000000)" 3.0)))
    (:then_1
      (bind _as_bp_actor_tile (Variables|Reference|GetAs%20BP%20Actor%20Tile)
        (:then
          (Default|EventTilePlayerStateRemove _as_bp_actor_tile PlayerState)
          (Variables|Reference|SetAs%20BP%20Actor%20Tile 0))
        (:else)))))

(event Custom|EventPlayerControllerAddPlayerStateLocal
  (params (Actor :type Actor%20Object%20Reference))
  (Variables|Reference|GetAs%20BP%20Actor%20Tile
    (:then
      (CallFunction|EventPlayerControllerRemovePlayerStateLocal))
    (:else
      _))
  (bind _asbp_actor_tile (Utilities|Casting|CastToBP_Actor_Tile Actor))
  (bind _output_get (Variables|Reference|SetAs%20BP%20Actor%20Tile _asbp_actor_tile))
  (CallFunction|EventPlayerControllerAddPlayerStateServer _output_get (Variables|/Script/Engine.Controller|GetPlayerState (Game|GetPlayerController 0))))

(event Custom|EventPlayerControllerRemovePlayerStateLocal
  (Utilities|FlowControl|Sequence
    (:then_0
      (if (Variables|Debug|GetbShowDebug?)
        (Development|PrintString "BP_PC_Gameplay - EVENT Remove PlayerState Local" true true "(R=0.000000,G=0.660000,B=1.000000,A=1.000000)" 3.0)))
    (:then_1
      (Variables|Reference|GetAs%20BP%20Actor%20Tile
        (:then
          (CallFunction|EventPlayerControllerRemovePlayerStateServer (Variables|/Script/Engine.Controller|GetPlayerState (Game|GetPlayerController 0)))
          (Variables|Reference|SetAs%20BP%20Actor%20Tile 0))
        (:else)))))

(event Input|EnhancedActionEvents|EnhancedInputActionIA_Tile_Primary
  (params (ActionValue :type Boolean) (ElapsedSeconds :type Float%20%28double-precision%29) (TriggeredSeconds :type Float%20%28double-precision%29) (InputAction :type Input%20Action%20Object%20Reference :default "/Game/SpawnTile/Gameplay/Player/Input/Actions/Tile/IA_Tile_Primary.IA_Tile_Primary"))
  (bind (_hit _hitactor) (CallFunction|GetActorUnderCursorbyChannel "TraceTypeQuery4"))
  (:Started
    (if _hit
      (bind _as_bp_actor_tile (Variables|Reference|GetAs%20BP%20Actor%20Tile)
        (:then
          (if (== _as_bp_actor_tile _hitactor)
            (CallFunction|EventPlayerControllerRemovePlayerStateLocal)
            (else
              (CallFunction|EventPlayerControllerRemovePlayerStateLocal)
              (CallFunction|EventPlayerControllerAddPlayerStateLocal _hitactor))))
        (:else
          (CallFunction|EventPlayerControllerAddPlayerStateLocal _hitactor))))))

(event Input|EnhancedActionEvents|EnhancedInputActionIA_Tile_Secondary
  (params (ActionValue :type Boolean) (ElapsedSeconds :type Float%20%28double-precision%29) (TriggeredSeconds :type Float%20%28double-precision%29) (InputAction :type Input%20Action%20Object%20Reference :default "/Game/SpawnTile/Gameplay/Player/Input/Actions/Tile/IA_Tile_Secondary.IA_Tile_Secondary"))
  (:Started
    (Utilities|FlowControl|Sequence
      (:then_0
        (if (Variables|Debug|GetbShowDebug?)
          (Development|PrintString "BP_PC_Gameplay - EVENT Cancel Tile On SERVER" true true "(R=0.000000,G=0.660000,B=1.000000,A=1.000000)" 3.0)))
      (:then_1
        (CallFunction|EventPlayerControllerRemovePlayerStateLocal)))))

(event Custom|EventPlayerControllerInitHUD
  (Utilities|FlowControl|Sequence
    (:then_0
      (if (Variables|Debug|GetbShowDebug?)
        (Development|PrintString "BP_PS_Gameplay - EVENT Init HUD" true true "(R=0.000000,G=0.660000,B=1.000000,A=1.000000)" 3.0)))
    (:then_1
      (bind _asbp_hud_gameplay (Utilities|Casting|CastToBP_HUD_Gameplay (HUD|GetHUD)))
      (Variables|Reference|SetAs%20BP%20HUD%20Gameplay _asbp_hud_gameplay))))

(event Custom|EventPlayerControllerUpdateAction
  (params (ActionData :type PDA%20Action%20Object%20Reference))
  (Utilities|FlowControl|Sequence
    (:then_0
      (if (Variables|Debug|GetbShowDebug?)
        (Development|PrintString "BP_PC_Gameplay - EVENT Select Action" true true "(R=0.000000,G=0.660000,B=1.000000,A=1.000000)" 3.0)))
    (:then_1
      (bind _output_get (Variables|Action|SetAction%20Data ActionData))
      (bind _asbp_aicontroller_unit (Utilities|Casting|CastToBP_AIController_Unit (AI|GetAIController 0)))
      (switch Utilities|FlowControl|Switch|SwitchonE_Phase (Variables|/Game/SpawnTile/Blueprints/Actions/Data/PDA_Action.PDA_Action_C|GetActive _output_get)
        (:NewEnumerator7
          (Default|EventAIControllerUpdateSpell _asbp_aicontroller_unit (Variables|/Game/SpawnTile/Blueprints/Actions/Data/PDA_Action.PDA_Action_C|GetClass _output_get)))
        (:NewEnumerator6
          (Default|EventAIControllerUpdatePreperation _asbp_aicontroller_unit (Variables|/Game/SpawnTile/Blueprints/Actions/Data/PDA_Action.PDA_Action_C|GetClass _output_get)))
        (:NewEnumerator3
          (Default|EventAIControllerUpdateDash _asbp_aicontroller_unit (Variables|/Game/SpawnTile/Blueprints/Actions/Data/PDA_Action.PDA_Action_C|GetClass _output_get)))
        (:NewEnumerator4
          (Default|EventAIControllerUpdateCombat _asbp_aicontroller_unit (Variables|/Game/SpawnTile/Blueprints/Actions/Data/PDA_Action.PDA_Action_C|GetClass _output_get)))
        (:NewEnumerator5
          (Default|EventAIControllerUpdateMovement _asbp_aicontroller_unit (Variables|/Game/SpawnTile/Blueprints/Actions/Data/PDA_Action.PDA_Action_C|GetClass _output_get)))))))

(event EventSetLoadout
  (params (Loadout :type F%20Loadout%20Structure))
  (Variables|Default|SetLoadout Loadout))

(fn ConstructionScript)

(fn GetActorUnderCursorbyChannel
  (params (TraceChannel :type ETraceTypeQuery%20Enum :default "TraceTypeQuery1"))
  (bind _hitresult (Game|Player|GetHitResultUnderCursorbyChannel TraceChannel true))
  (bind (_bblockinghit _binitialoverlap _time _distance _location _impactpoint _normal _impactnormal _physmat _hitactor) (Collision|BreakHitResult _hitresult))
  (return _bblockinghit _hitactor))

(fn OnRepasBPCharacterUnit
  (bind _as_bp_hud_gameplay (Variables|Reference|GetAs%20BP%20HUD%20Gameplay)
    (:then
      (Default|EventWBPHUDUpdateUnit _as_bp_hud_gameplay (Variables|Default|GetAs%20BP%20Character%20Unit_)))
    (:else)))

(fn OnRepLoadout
  (Variables|Reference|GetAs%20BP%20HUD%20Gameplay
    (:then)
    (:else)))

(fn GetLoadout
  (return ""))