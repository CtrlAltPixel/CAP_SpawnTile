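; Game state for a turn-based game that drives match, turn, phase and unit-action flow from player planning through resolve phases.
; Each resolve phase queues units whose AI controller holds a relevant action, then adds that action component to one unit at a time.
; Phase ends advance the enum, and turn end checks kill and turn limits.
; Phase replication broadcasts changes and shows HUD notifications; turn-start setup is unwired.
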(event `self.ReceiveBeginPlay`
  (`|ExecutionSequence`
    (:`then_0`
      (if (`self.bShowDebug?`)
        (`KismetSystemLibrary.PrintString` "BP_GS_Gameplay - EVENT BeginPlay" true true (struct :`G` 0.66 :`B` 1.0 :`A` 1.0) 3.0)))
    (:`then_1`
      (`KismetSystemLibrary.Delay` 3.0)
      (`self.EventGameStateMatchStart`))))

(event `EventGameStateMatchStart`
  (`|ExecutionSequence`
    (:`then_0`
      (if (`self.bShowDebug?`)
        (`KismetSystemLibrary.PrintString` "BP_GS_Gameplay - EVENT StartMatch" true true (struct :`G` 0.66 :`B` 1.0 :`A` 1.0) 3.0)))))

(event `EventGameStateMatchEnd`
  (`|ExecutionSequence`
    (:`then_0`
      (if (`self.bShowDebug?`)
        (`KismetSystemLibrary.PrintString` "BP_GS_Gameplay - EVENT EndMatch" true true (struct :`G` 0.66 :`B` 1.0 :`A` 1.0) 3.0)))))

(event `EventGameStateTurnStart`
  (`|ExecutionSequence`
    (:`then_0`
      (if (`self.bShowDebug?`)
        (`KismetSystemLibrary.PrintString` "BP_GS_Gameplay - EVENT Turn Start" true true (struct :`G` 0.66 :`B` 1.0 :`A` 1.0) 3.0)))))

(event `EventGameStateTurnEnd`
  (`|ExecutionSequence`
    (:`then_0`
      (if (`self.bShowDebug?`)
        (`KismetSystemLibrary.PrintString` "BP_GS_Gameplay - EVENT Turn End" true true (struct :`G` 0.66 :`B` 1.0 :`A` 1.0) 3.0)))
    (:`then_1`
      (bind _bsuccess_ (`self.Func_MaxKills`))
      (if _bsuccess_
        (`self.EventGameStateMatchEnd`)
        (else
          (bind _bsuccess__2 (`self.Func_MaxTurns`))
          (if _bsuccess__2
            (`self.EventGameStateMatchEnd`)))))))

(event `EventGameStatePhaseStart`
  (`|ExecutionSequence`
    (:`then_0`
      (if (`self.bShowDebug?`)
        (`KismetSystemLibrary.PrintString` (`KismetStringLibrary.Concat_StrStr` "BP_GS_Gameplay - EVENT PhaseStart - " (`|GetEnumeratorNameAsString` (`self.Phase`))) true true (struct :`G` 0.66 :`B` 1.0 :`A` 1.0) 3.0)))
    (:`then_1`
      (switch `/Game/SpawnTile/Gameplay/System/Enum/E_Phase` (`self.Phase`)
        (:`NewEnumerator7`
          _)
        (:`NewEnumerator6`
          _)
        (:`NewEnumerator3`
          _)
        (:`NewEnumerator4`
          _)
        (:`NewEnumerator2`
          _)
        (:`NewEnumerator5`
          _)
        (:`NewEnumerator1`
          _))
      (bind _unitstoaction (`self.Func_CreateUnitQue`))
      (set `self.UnitQue` _unitstoaction)
      (`self.EventGameStateActionStart`))))

(event `EventGameStateUpdatePhase`
  (params (Phase :type "/Game/SpawnTile/Gameplay/System/Enum/E_Phase Enum" :default "NewEnumerator9"))
  (`|ExecutionSequence`
    (:`then_0`
      (if (`self.bShowDebug?`)
        (`KismetSystemLibrary.PrintString` "BP_GS_Gameplay - EVENT Update Phase" true true (struct :`G` 0.66 :`B` 1.0 :`A` 1.0) 3.0)))
    (:`then_1`
      (set `self.Phase` Phase))))

(event `EventGameStateUpdateReadyTimer`
  (bind _readytime (`self.ReadyTime`))
  (`|ExecutionSequence`
    (:`then_0`
      (if (`self.bShowDebug?`)
        (`KismetSystemLibrary.PrintString` "BP_GS_Gameplay - EVENT Update Ready Timer" true true (struct :`G` 0.66 :`B` 1.0 :`A` 1.0) 3.0)))
    (:`then_1`
      (if (> _readytime 0)
        (set `self.ReadyTime` (- _readytime 1))))))

(event `EventGameStatePhaseEnd`
  (`|ExecutionSequence`
    (:`then_0`
      (if (`self.bShowDebug?`)
        (`KismetSystemLibrary.PrintString` "BP_GS_Gameplay - EVENT PhaseEnd" true true (struct :`G` 0.66 :`B` 1.0 :`A` 1.0) 3.0)))
    (:`then_1`
      (switch `/Game/SpawnTile/Gameplay/System/Enum/E_Phase` (`self.Phase`)
        (:`NewEnumerator0`
          (`self.Func_ProgressToNextPhase`))
        (:`NewEnumerator7`
          (`self.Func_ProgressToNextPhase` :!label _label))
        (:`NewEnumerator6`
          (goto _label))
        (:`NewEnumerator3`
          (goto _label))
        (:`NewEnumerator4`
          (goto _label))
        (:`NewEnumerator2`
          (goto _label))
        (:`NewEnumerator5`
          (goto _label))
        (:`NewEnumerator1`
          (`self.EventGameStateTurnEnd`))))))

(event `EventGameStateActionStart`
  (`|ExecutionSequence`
    (:`then_0`
      (`/Game/SpawnTile/Gameplay/System/CommonFunctionLibrary.DebugMessage` "BP_GS_Gameplay - EVENT ActionStart" (`self.bShowDebug?`)))
    (:`then_1`
      (bind _output_get (set `self.CurrentUnit` (`|GetArrayItem` (`self.UnitQue`))))
      (bind _asbp_aicontroller_unit (cast `/Game/SpawnTile/Gameplay/Unit/AI/BP_AIController_Unit` (`AIBlueprintHelperLibrary.GetAIController` _output_get)))
      (switch `/Game/SpawnTile/Gameplay/System/Enum/E_Phase` (`self.Phase`)
        (:`NewEnumerator7`
          (`|AddComponentByClass` (`self.CurrentUnit`) (`/Game/SpawnTile/Gameplay/Unit/AI/BP_AIController_Unit.SpellAction` _asbp_aicontroller_unit)))
        (:`NewEnumerator6`
          (`|AddComponentByClass` (`self.CurrentUnit`) (`/Game/SpawnTile/Gameplay/Unit/AI/BP_AIController_Unit.PreperationAction` _asbp_aicontroller_unit)))
        (:`NewEnumerator3`
          (`|AddComponentByClass` (`self.CurrentUnit`) (`/Game/SpawnTile/Gameplay/Unit/AI/BP_AIController_Unit.DashAction` _asbp_aicontroller_unit)))
        (:`NewEnumerator4`
          (`|AddComponentByClass` (`self.CurrentUnit`) (`/Game/SpawnTile/Gameplay/Unit/AI/BP_AIController_Unit.CombatAction` _asbp_aicontroller_unit)))
        (:`NewEnumerator2`
          (`|AddComponentByClass` (`self.CurrentUnit`) (`/Game/SpawnTile/Gameplay/Unit/AI/BP_AIController_Unit.DeathAction` _asbp_aicontroller_unit)))
        (:`NewEnumerator5`
          (`|AddComponentByClass` (`self.CurrentUnit`) (`/Game/SpawnTile/Gameplay/Unit/AI/BP_AIController_Unit.MovementAction` _asbp_aicontroller_unit)))))))

(event `EventGameStateOnActionUpdate`
  (`|ExecutionSequence`
    (:`then_0`
      (`/Game/SpawnTile/Gameplay/System/CommonFunctionLibrary.DebugMessage` "BP_GS_Gameplay - EVENT ActionEnd"))
    (:`then_1`
      (bind _asbp_character_unit (cast `/Game/SpawnTile/Gameplay/Unit/BP_Character_Unit` (`self.CurrentUnit`)))
      (add `/Game/SpawnTile/Gameplay/Unit/BP_Character_Unit.OnAnimMontageEnd` _asbp_character_unit (`|CreateDelegate` :!event `EventGameStateActionEnd`))
      (`/Game/SpawnTile/Gameplay/Unit/BP_Character_Unit.MULTIPlayAnimMontage` _asbp_character_unit null))))

(event `EventGameStateActionEnd`
  (`|ExecutionSequence`
    (:`then_0`
      (`/Game/SpawnTile/Gameplay/System/CommonFunctionLibrary.DebugMessage` "BP_GS_Gameplay - EVENT ActionEnd" (`self.bShowDebug?`)))
    (:`then_1`
      (`KismetArrayLibrary.Array_RemoveItem` (`self.UnitQue`) (`self.CurrentUnit`))
      (set `self.CurrentUnit` null)
      (if (`KismetArrayLibrary.Array_IsEmpty` (`self.UnitQue`))
        (`self.EventGameStatePhaseEnd`)
        (else
          (`self.EventGameStateActionStart`))))))

(fn `Func_AllPlayersReady`
  (returns (`bAllReady?` :type Boolean))
  (locals (Local_AllReady :type Boolean))
  (for _array_element (`self.PlayerArray`)
    (bind _asbp_ps_gameplay (cast `/Game/SpawnTile/Gameplay/Player/State/BP_PS_Gameplay` _array_element))
    (if (`/Game/SpawnTile/Gameplay/Player/State/BP_PS_Gameplay.bIsReady?` _asbp_ps_gameplay)
      (set `local.Local_AllReady` true)
      (else
        (return false))))
  (return (`local.Local_AllReady`)))

(fn `Func_CreateUnitQue`
  (returns (UnitsToAction :type "Array of Pawn Object Reference"))
  (locals (Local_Unit :type "/Game/SpawnTile/Gameplay/Unit/BP_Character_Unit Object Reference") (Local_AIController :type "/Game/SpawnTile/Gameplay/Unit/AI/BP_AIController_Unit Object Reference") (Local_UnitQue :type "Array of Pawn Object Reference"))
  (`KismetArrayLibrary.Array_Clear` (`local.Local_UnitQue`))
  (bind _outactors (`GameplayStatics.GetAllActorsOfClass` "/Game/SpawnTile/Gameplay/Unit/BP_Character_Unit.BP_Character_Unit_C"))
  (for _array_element _outactors
    (bind _output_get (set `local.Local_Unit` _array_element))
    (bind _asbp_aicontroller_unit (cast `/Game/SpawnTile/Gameplay/Unit/AI/BP_AIController_Unit` (`AIBlueprintHelperLibrary.GetAIController` _output_get)))
    (set `local.Local_AIController` _asbp_aicontroller_unit)
    (switch `/Game/SpawnTile/Gameplay/System/Enum/E_Phase` (`self.Phase`)
      (:`NewEnumerator7`
        (bind _local_aicontroller (`local.Local_AIController`)
          (:`then`
            (`/Game/SpawnTile/Gameplay/Unit/AI/BP_AIController_Unit.SpellAction` _local_aicontroller
              (:`then`
                (`KismetArrayLibrary.Array_Add` (`local.Local_UnitQue`) (`local.Local_Unit`)))
              (:`else`)))
          (:`else`)))
      (:`NewEnumerator6`
        (bind _local_aicontroller_2 (`local.Local_AIController`)
          (:`then`
            (`/Game/SpawnTile/Gameplay/Unit/AI/BP_AIController_Unit.SpellAction` _local_aicontroller_2
              (:`then`
                (`KismetArrayLibrary.Array_Add` (`local.Local_UnitQue`) (`local.Local_Unit`)))
              (:`else`)))
          (:`else`)))
      (:`NewEnumerator3`
        (bind _local_aicontroller_3 (`local.Local_AIController`)
          (:`then`
            (`/Game/SpawnTile/Gameplay/Unit/AI/BP_AIController_Unit.DashAction` _local_aicontroller_3
              (:`then`
                (`KismetArrayLibrary.Array_Add` (`local.Local_UnitQue`) (`local.Local_Unit`)))
              (:`else`)))
          (:`else`)))
      (:`NewEnumerator4`
        (bind _local_aicontroller_4 (`local.Local_AIController`)
          (:`then`
            (`/Game/SpawnTile/Gameplay/Unit/AI/BP_AIController_Unit.CombatAction` _local_aicontroller_4
              (:`then`
                (`KismetArrayLibrary.Array_Add` (`local.Local_UnitQue`) (`local.Local_Unit`)))
              (:`else`)))
          (:`else`)))
      (:`NewEnumerator2`
        (bind _local_aicontroller_5 (`local.Local_AIController`)
          (:`then`
            (`/Game/SpawnTile/Gameplay/Unit/AI/BP_AIController_Unit.DeathAction` _local_aicontroller_5
              (:`then`
                (`KismetArrayLibrary.Array_Add` (`local.Local_UnitQue`) (`local.Local_Unit`)))
              (:`else`)))
          (:`else`)))
      (:`NewEnumerator5`
        (bind _local_aicontroller_6 (`local.Local_AIController`)
          (:`then`
            (`/Game/SpawnTile/Gameplay/Unit/AI/BP_AIController_Unit.MovementAction` _local_aicontroller_6
              (:`then`
                (`KismetArrayLibrary.Array_Add` (`local.Local_UnitQue`) (`local.Local_Unit`)))
              (:`else`)))
          (:`else`)))))
  (return (`local.Local_UnitQue`)))

(fn `Func_MaxKills`
  (returns (`bSuccess?` :type Boolean))
  (return (or (> 0 (`self.Setting_MaxKills`)) (> 0 (`self.Setting_MaxKills`)))))

(fn `Func_MaxTurns`
  (returns (`bSuccess?` :type Boolean))
  (return (>= (`self.TurnCount`) (`self.Setting_MaxTurns`))))

(fn `Func_ProgressToNextPhase`
  (bind _result (`/Engine/EditorBlueprintResources/StandardMacros.IncrementInt` (`KismetMathLibrary.Conv_ByteToInt` (`self.Phase`)))
    (:`  `
      (`self.EventGameStateUpdatePhase` (cast `/Game/SpawnTile/Gameplay/System/Enum/E_Phase` (`KismetMathLibrary.Conv_IntToByte` (mod _result (enumcount `/Game/SpawnTile/Gameplay/System/Enum/E_Phase`))))))))

(fn `Func_ShowNotificationWidget`
  (params (Title :type Text) (Content :type Text) (DisplayTime :type "Float (single-precision)"))
  (bind _asbp_hud_gameplay (cast `/Game/SpawnTile/Gameplay/HUD/BP_HUD_Gameplay` (`PlayerController.GetHUD` (`GameplayStatics.GetPlayerController` 0))))
  (`/Game/SpawnTile/Gameplay/HUD/Notification/WBP_Notification.Func_CreateNotification` (`/Game/SpawnTile/Gameplay/HUD/BP_HUD_Gameplay.AsWB_Notification` _asbp_hud_gameplay) Title Content DisplayTime))

(fn `Func_UpdateTurnCount`
  (set `self.TurnCount` (+ (`self.TurnCount`) 1)))

(fn `OnRep_Phase`
  (`self.OnPhaseUpdate` (`self.Phase`))
  (bind _asbp_hud_gameplay (cast `/Game/SpawnTile/Gameplay/HUD/BP_HUD_Gameplay` (`PlayerController.GetHUD` (`GameplayStatics.GetPlayerController` 0))))
  (`/Game/SpawnTile/Gameplay/HUD/Notification/WBP_Notification.Func_CreateNotification` (`/Game/SpawnTile/Gameplay/HUD/BP_HUD_Gameplay.AsWB_Notification` _asbp_hud_gameplay) (`KismetTextLibrary.Conv_StringToText` (`|GetEnumeratorNameAsString` (`self.Phase`))) "" 3.0))

(fn `UserConstructionScript`)