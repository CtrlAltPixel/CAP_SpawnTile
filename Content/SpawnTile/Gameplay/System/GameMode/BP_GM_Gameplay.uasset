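; Gameplay game mode that tracks player controllers and spawns units assigned to a commanding player.
; Login and logout maintain the controller list, while controller swaps copy the loadout message to the new controller and add it.
; Unit spawn creates a BP_Character_Unit with its command controller, spawns its default controller, then announces it through CallOnUnitSpawn.
; BeginPlay binds to unit deaths; the unit-died and AI-query events only emit debug messages.
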(event `self.ReceiveBeginPlay`
  (`|ExecutionSequence`
    (:`then_0`
      (`/Game/SpawnTile/Gameplay/System/CommonFunctionLibrary.DebugMessage` "BP_GM_Gameplay - Event Begin Play" (`self.bShowDebug?`)))
    (:`then_1`
      (add `self.OnUnitDied` (`|CreateDelegate` :!event `EventGameModeUnitDied`)))))

(event `self.K2_PostLogin`
  (params (NewPlayer :type "PlayerController Object Reference"))
  (`|ExecutionSequence`
    (:`then_0`
      (`/Game/SpawnTile/Gameplay/System/CommonFunctionLibrary.DebugMessage` "BP_GM_Gameplay - Event  On Post Login" (`self.bShowDebug?`)))
    (:`then_1`
      (`KismetArrayLibrary.Array_Add` (`self.AllPlayerControllers`) NewPlayer))))

(event `self.K2_OnSwapPlayerControllers`
  (params (OldPC :type "PlayerController Object Reference") (NewPC :type "PlayerController Object Reference"))
  (`|ExecutionSequence`
    (:`then_0`
      (`/Game/SpawnTile/Gameplay/System/CommonFunctionLibrary.DebugMessage` "BP_GM_Gameplay - Event Swap Player Controllers" (`self.bShowDebug?`)))
    (:`then_1`
      (bind _loadout (message `/Game/SpawnTile/Blueprints/Loadout/Interface/BPI_Loadout.GetLoadout` OldPC))
      (message `/Game/SpawnTile/Blueprints/Loadout/Interface/BPI_Loadout.SetLoadout` NewPC _loadout)
      (`KismetArrayLibrary.Array_Add` (`self.AllPlayerControllers`) NewPC))))

(event `EventGameModeUnitSpawn`
  (params (SpawnTransform :type "Transform Structure") (PlayerController :type "PlayerController Object Reference"))
  (`|ExecutionSequence`
    (:`then_0`
      (`/Game/SpawnTile/Gameplay/System/CommonFunctionLibrary.DebugMessage` "BP_GM_Gameplay - Event Unit Spawn" (`self.bShowDebug?`)))
    (:`then_1`
      (bind _returnvalue (`|SpawnActorFromClass` "/Game/SpawnTile/Gameplay/Unit/BP_Character_Unit.BP_Character_Unit_C" SpawnTransform "AdjustIfPossibleButAlwaysSpawn" "MultiplyWithRoot" null PlayerController null))
      (`Pawn.SpawnDefaultController` _returnvalue)
      (`self.OnUnitSpawn` _returnvalue))))

(event `EventGameModeUnitDied` :!signature `self.OnUnitDied`
  (params (Character :type "Character Object Reference"))
  (`|ExecutionSequence`
    (:`then_0`
      (`/Game/SpawnTile/Gameplay/System/CommonFunctionLibrary.DebugMessage` "BP_GM_Gameplay - Event Unit Died" (`self.bShowDebug?`)))))

(event `EventGameModeQueryAIUnits`
  (`|ExecutionSequence`
    (:`then_0`
      (`/Game/SpawnTile/Gameplay/System/CommonFunctionLibrary.DebugMessage` "BP_GM_Gameplay - Event Query AIUnits"))))

(event `self.K2_OnLogout`
  (params (ExitingController :type "Controller Object Reference"))
  (`|ExecutionSequence`
    (:`then_0`
      (`/Game/SpawnTile/Gameplay/System/CommonFunctionLibrary.DebugMessage` "BP_GM_Gameplay - Event On Logout" (`self.bShowDebug?`)))
    (:`then_1`
      (bind _asplayer_controller (cast `PlayerController` ExitingController))
      (`KismetArrayLibrary.Array_RemoveItem` (`self.AllPlayerControllers`) _asplayer_controller))))

(fn `UserConstructionScript`)