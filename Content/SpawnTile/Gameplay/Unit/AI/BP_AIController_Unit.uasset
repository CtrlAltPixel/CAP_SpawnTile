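; AI controller for gameplay units that holds the unit's current action for each phase: spell, preparation, dash, combat, death and movement.
; Each update event logs an optional debug message, then stores the passed action in its matching variable.
; The graph contains no decision logic; it only receives and caches these actions, and Tick is unused.
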(event `self.ReceiveBeginPlay`
  (`|ExecutionSequence`
    (:`then_0`
      (`/Game/SpawnTile/Gameplay/System/CommonFunctionLibrary.DebugMessage` "BP_AIController_Gameplay - EVENT Begin Play" (`self.bShowDebug?`)))))

(event `EventAIControllerUpdateSpell`
  (params (PlanningAction :type "/Game/SpawnTile/Blueprints/Actions/BP_AC_Action Class Reference"))
  (`|ExecutionSequence`
    (:`then_0`
      (`/Game/SpawnTile/Gameplay/System/CommonFunctionLibrary.DebugMessage` "BP_AIController_Gameplay - EVENT Update Spell" (`self.bShowDebug?`)))
    (:`then_1`
      (set `self.SpellAction` PlanningAction))))

(event `EventAIControllerUpdatePreperation`
  (params (PlanningAction :type "/Game/SpawnTile/Blueprints/Actions/BP_AC_Action Class Reference"))
  (`|ExecutionSequence`
    (:`then_0`
      (`/Game/SpawnTile/Gameplay/System/CommonFunctionLibrary.DebugMessage` "BP_AIController_Gameplay - EVENT Update Planning" (`self.bShowDebug?`)))
    (:`then_1`
      (set `self.PreperationAction` PlanningAction))))

(event `EventAIControllerUpdateDash`
  (params (DashAction :type "/Game/SpawnTile/Blueprints/Actions/BP_AC_Action Class Reference"))
  (`|ExecutionSequence`
    (:`then_0`
      (`/Game/SpawnTile/Gameplay/System/CommonFunctionLibrary.DebugMessage` "BP_AIController_Gameplay - EVENT Update Dash" (`self.bShowDebug?`)))
    (:`then_1`
      (set `self.DashAction` DashAction))))

(event `EventAIControllerUpdateCombat`
  (params (CombatAction :type "/Game/SpawnTile/Blueprints/Actions/BP_AC_Action Class Reference"))
  (`|ExecutionSequence`
    (:`then_0`
      (`/Game/SpawnTile/Gameplay/System/CommonFunctionLibrary.DebugMessage` "BP_AIController_Gameplay - EVENT Update Combat" (`self.bShowDebug?`)))
    (:`then_1`
      (set `self.CombatAction` CombatAction))))

(event `EventAIControllerUpdateDeath`
  (params (DeathAction :type "/Game/SpawnTile/Blueprints/Actions/BP_AC_Action Class Reference"))
  (`|ExecutionSequence`
    (:`then_0`
      (`/Game/SpawnTile/Gameplay/System/CommonFunctionLibrary.DebugMessage` "BP_AIController_Gameplay - EVENT Update Combat" (`self.bShowDebug?`)))
    (:`then_1`
      (set `self.DeathAction` DeathAction))))

(event `EventAIControllerUpdateMovement`
  (params (MovementAction :type "/Game/SpawnTile/Blueprints/Actions/BP_AC_Action Class Reference"))
  (`|ExecutionSequence`
    (:`then_0`
      (`/Game/SpawnTile/Gameplay/System/CommonFunctionLibrary.DebugMessage` "BP_AIController_Gameplay - EVENT Update Movement" (`self.bShowDebug?`)))
    (:`then_1`
      (set `self.MovementAction` MovementAction))))

(fn `UserConstructionScript`)