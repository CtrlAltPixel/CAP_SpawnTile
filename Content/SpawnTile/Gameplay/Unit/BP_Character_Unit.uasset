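; BP_Character_Unit is a replicated unit character that initializes from a unit data asset and reports its lifecycle to gameplay classes.
; On possession, it registers with the commanding player controller if valid, then initializes using the debug data asset and a fixed team.
; RepNotifies apply the mesh and pass team changes to the team component.
; It also notifies the game mode of death and plays multicast montages with begin/end callbacks.
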(event `self.ReceiveBeginPlay`
  (`|ExecutionSequence`
    (:`then_0`
      (`/Game/SpawnTile/Gameplay/System/CommonFunctionLibrary.DebugMessage` "BP Character Unit - EVENT BeginPlay" (`self.bShowDebug?`)))
    (:`then_1`
      (`PrimitiveComponent.SetCollisionResponseToChannel` (`self.CapsuleComponent`) "ECC_GameTraceChannel1" "ECR_Block")
      (`PrimitiveComponent.SetReceivesDecals` (`self.Mesh`) false))))

(event `self.ReceivePossessed`
  (params (NewController :type "Controller Object Reference"))
  (`|ExecutionSequence`
    (:`then_0`
      (`/Game/SpawnTile/Gameplay/System/CommonFunctionLibrary.DebugMessage` "BP Character Unit - Event Possessed" (`self.bShowDebug?`)))
    (:`then_1`
      (`self.CommandPlayerController`
        (:`then`
          (`self.EventUnitRegisterSpawn`)
          (`self.EventUnitInit` "/Game/SpawnTile/Gameplay/Unit/Data/DA_Unit_Debug.DA_Unit_Debug"))
        (:`else`
          (`self.EventUnitInit` "/Game/SpawnTile/Gameplay/Unit/Data/DA_Unit_Debug.DA_Unit_Debug"))))))

(event `EventUnitRegisterSpawn`
  (`|ExecutionSequence`
    (:`then_0`
      (`/Game/SpawnTile/Gameplay/System/CommonFunctionLibrary.DebugMessage` "BP Character Unit - EVENT Unit RegisterSpawn" (`self.bShowDebug?`)))
    (:`then_1`
      (bind _commandplayercontroller (`self.CommandPlayerController`)
        (:`then`
          (bind _asbp_pc_gameplay (cast `/Game/SpawnTile/Gameplay/Player/Controller/BP_PC_Gameplay` _commandplayercontroller))
          (`/Game/SpawnTile/Gameplay/Player/Controller/BP_PC_Gameplay.EventUnitUpdateOnPlayerController` _asbp_pc_gameplay self))
        (:`else`)))))

(event `EventUnitRegisterDeath`
  (`|ExecutionSequence`
    (:`then_0`
      (`/Game/SpawnTile/Gameplay/System/CommonFunctionLibrary.DebugMessage` "BP Character Unit - EVENT Register Death" (`self.bShowDebug?`)))
    (:`then_1`
      (`self.As_BP_GM_Gameplay`
        (:`then`
          _)
        (:`else`
          (bind _asbp_gm_gameplay (cast `/Game/SpawnTile/Gameplay/System/GameMode/BP_GM_Gameplay` (`GameplayStatics.GetGameMode`)))
          (set `self.As_BP_GM_Gameplay` _asbp_gm_gameplay)))
      (`/Game/SpawnTile/Gameplay/System/GameMode/BP_GM_Gameplay.EventGameModeUnitDied` (`self.As_BP_GM_Gameplay`) self))))

(event `EventUnitInit`
  (params (UnitData :type "/Game/SpawnTile/Gameplay/Unit/Data/PDA_Unit Object Reference"))
  (`|ExecutionSequence`
    (:`then_0`
      (`/Game/SpawnTile/Gameplay/System/CommonFunctionLibrary.DebugMessage` "BP Character Unit - EVENT Unit Initialize" (`self.bShowDebug?`)))
    (:`then_1`
      (set `self.UnitData` UnitData)
      (bind _unitdata (`self.UnitData`)
        (:`then`
          (set `self.Name` (`/Game/SpawnTile/Gameplay/Unit/Data/PDA_Unit.Name` _unitdata))
          (set `self.UnitMesh` (`/Game/SpawnTile/Gameplay/Unit/Data/PDA_Unit.Mesh` _unitdata))
          (set `self.Team` "NewEnumerator0"))
        (:`else`)))))

(event `MULTIPlayAnimMontage`
  (params (AnimMontage :type "AnimMontage Object Reference"))
  (`|ExecutionSequence`
    (:`then_0`
      (`/Game/SpawnTile/Gameplay/System/CommonFunctionLibrary.DebugMessage` "BP Character Unit - EVENT AnimMontage" (`self.bShowDebug?`)))
    (:`then_1`
      (bind _output_get (set `self.AsCurrentAnimMontage` AnimMontage))
      (`|PlayMontage` (`self.Mesh`) _output_get
        (:`then`
          (`self.OnAimMontageBegin`))
        (:`OnCompleted`
          (set `self.AsCurrentAnimMontage` null :!label _label)
          (`self.OnAnimMontageEnd`))
        (:`OnBlendOut`
          (goto _label))
        (:`OnInterrupted`
          (goto _label))))))

(fn `OnRep_Name`)

(fn `OnRep_Team`
  (`/Game/SpawnTile/Blueprints/Team/BP_AC_Team.UpdateTeam` (`self.BP_AC_Team`) (`self.Team`)))

(fn `OnRep_UnitMesh`
  (`SkeletalMeshComponent.SetSkeletalMeshAsset` (`self.Mesh`) (`self.UnitMesh`)))

(fn `SetActorHidden`
  (params (bNewHidden :type Boolean))
  (`self.SetActorHiddenInGame` bNewHidden)
  (`self.SetActorEnableCollision` (not bNewHidden)))

(fn `UserConstructionScript`)