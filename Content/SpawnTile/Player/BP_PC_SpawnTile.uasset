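; Player controller for the SpawnTile game that handles tile selection, Alive/Dead status and character spawning.
; Cursor traces select tiles, releasing the previous one; character clicks only print debug text.
; Status updates swap Character and Dead input contexts, toggle the HUD's dead overlay and notify listeners.
; Debug keys set status through the game mode or spawn a character at the PlayerState transform, clearing tile selection and setting Dead.
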(event Custom|UpdatePlayerStatus
  (params (Selection :type E_PlayerStatus%20Enum :default "NewEnumerator0"))
  (bind _output_get (Variables|Default|SetPlayerStatus Selection))
  (Default|CallOnStatusChanged _output_get)
  (switch Utilities|FlowControl|Switch|SwitchonE_PlayerStatus _output_get
    (:NewEnumerator1
      (Input|RemoveMappingContext (PlayerController|LocalPlayerSubsystems|GetEnhancedInputLocalPlayerSubsystem) "/Game/SpawnTile/Input/IMC_Dead.IMC_Dead" "(bIgnoreAllPressedKeysUntilRelease=True,bForceImmediately=False,bNotifyUserSettings=False)")
      (Input|AddMappingContext (PlayerController|LocalPlayerSubsystems|GetEnhancedInputLocalPlayerSubsystem) "/Game/SpawnTile/Input/IMC_Character.IMC_Character" 0 "(bIgnoreAllPressedKeysUntilRelease=True,bForceImmediately=False,bNotifyUserSettings=False)")
      (bind _as_bp_hud_spawn_tile (Variables|Default|GetAs%20BP%20HUD%20Spawn%20Tile)
        (:then
          (Default|RemoveDeadOverlay _as_bp_hud_spawn_tile))
        (:else)))
    (:NewEnumerator2
      (Input|RemoveMappingContext (PlayerController|LocalPlayerSubsystems|GetEnhancedInputLocalPlayerSubsystem) "/Game/SpawnTile/Input/IMC_Character.IMC_Character" "(bIgnoreAllPressedKeysUntilRelease=True,bForceImmediately=False,bNotifyUserSettings=False)")
      (Input|AddMappingContext (PlayerController|LocalPlayerSubsystems|GetEnhancedInputLocalPlayerSubsystem) "/Game/SpawnTile/Input/IMC_Dead.IMC_Dead" 0 "(bIgnoreAllPressedKeysUntilRelease=True,bForceImmediately=False,bNotifyUserSettings=False)")
      (bind _as_bp_hud_spawn_tile_2 (Variables|Default|GetAs%20BP%20HUD%20Spawn%20Tile)
        (:then
          (Default|ShowDeadOverlay _as_bp_hud_spawn_tile_2))
        (:else)))))

(event Custom|SERVER_SpawnCharacter
  (bind _asbp_ps_spawn_tile (Utilities|Casting|CastToBP_PS_SpawnTile (Game|GetPlayerState 0)))
  (bind _returnvalue (Game|SpawnActorfromClass "/Game/SpawnTile/Character/Player/BP_Character_Player.BP_Character_Player_C" (Variables|/Game/SpawnTile/Player/BP_PS_SpawnTile.BP_PS_SpawnTile_C|GetTransform _asbp_ps_spawn_tile) "AlwaysSpawn" "MultiplyWithRoot" 0 self 0))
  (Variables|Default|SetControlledUnit _returnvalue)
  (bind _asbp_actor_tile (Utilities|Casting|CastToBP_Actor_Tile (Variables|Default|GetAsSelectedActor)))
  (Default|RemovePlayerSelection _asbp_actor_tile self)
  (bind _asbp_gm_spawn_tiler (Utilities|Casting|CastToBP_GM_SpawnTiler (Game|GetGameMode)))
  (Default|SetPlayerStatus _asbp_gm_spawn_tiler self "NewEnumerator2"))

(event Input|EnhancedActionEvents|EnhancedInputActionIA_Character
  (params (ActionValue :type Boolean) (ElapsedSeconds :type Float%20%28double-precision%29) (TriggeredSeconds :type Float%20%28double-precision%29) (InputAction :type Input%20Action%20Object%20Reference :default "/Game/SpawnTile/Input/Actions/IA_Character.IA_Character"))
  (bind (_hit _hitactor) (CallFunction|GetActorUnderCursor))
  (:Started
    (if _hit
      (if (Class|GameplayStatics|ObjectIsA _hitactor "/Game/SpawnTile/Character/BP_Character_SpawnTile.BP_Character_SpawnTile_C")
        (Development|PrintString "ShouldHaveACharacter")
        (else
          (Development|PrintString "Not ACharacter")))
      (else
        (Development|PrintString "NoCharacterActor")))))

(event Input|EnhancedActionEvents|EnhancedInputActionIA_SelectSpawn
  (params (ActionValue :type Boolean) (ElapsedSeconds :type Float%20%28double-precision%29) (TriggeredSeconds :type Float%20%28double-precision%29) (InputAction :type Input%20Action%20Object%20Reference :default "/Game/SpawnTile/Input/Actions/IA_SelectSpawn.IA_SelectSpawn"))
  (bind (_hit _hitactor) (CallFunction|GetActorUnderCursor))
  (:Started
    (if _hit
      (if (Class|GameplayStatics|ObjectIsA _hitactor "/Game/SpawnTile/Tile/BP_Actor_Tile.BP_Actor_Tile_C")
        (CallFunction|SetSelectedTile _hitactor)
        (Development|PrintString "Should have Tile")
        (else
          (Development|PrintString "NoTile")))
      (else
        (Development|PrintString "NoTileActor")))))

(event EventBeginPlay
  (bind _returnvalue (PlayerController|LocalPlayerSubsystems|GetEnhancedInputLocalPlayerSubsystem))
  (if (Pawn|IsLocalPlayerController)
    ;[0.05098 0.05098 0.05098] Add Mapping Context
    (Utilities|IsValid _returnvalue
      (:Is%20Valid
        (Input|AddMappingContext _returnvalue "/Game/SpawnTile/Input/IMC_Camera.IMC_Camera" 0 "(bIgnoreAllPressedKeysUntilRelease=True,bForceImmediately=False,bNotifyUserSettings=False)")
        (Input|AddMappingContext _returnvalue "/Game/SpawnTile/Input/IMC_Character.IMC_Character" 0 "(bIgnoreAllPressedKeysUntilRelease=True,bForceImmediately=False,bNotifyUserSettings=False)")
        (CallFunction|InitCasts)))))

(event Input|KeyboardEvents|DebugKey3
  (params (Key :type Key%20Structure) (ActionValue :type Input%20Action%20Value%20Structure))
  (:Pressed
    (CallFunction|SERVERSpawnCharacter)))

(event Input|KeyboardEvents|1
  (params (Key :type Key%20Structure))
  (:Pressed
    (bind _asbp_gm_spawn_tiler (Utilities|Casting|CastToBP_GM_SpawnTiler (Game|GetGameMode)))
    (Default|SetPlayerStatus _asbp_gm_spawn_tiler self "NewEnumerator2")
    (Development|PrintString (Utilities|String|EnumtoString (Variables|Default|GetPlayerStatus)))))

(event Input|KeyboardEvents|2
  (params (Key :type Key%20Structure))
  (:Pressed
    (bind _asbp_gm_spawn_tiler (Utilities|Casting|CastToBP_GM_SpawnTiler (Game|GetGameMode)))
    (Default|SetPlayerStatus _asbp_gm_spawn_tiler self "NewEnumerator1")
    (Development|PrintString (Utilities|String|EnumtoString (Variables|Default|GetPlayerStatus)))))

(fn ConstructionScript)

(fn Moveto
  (params (Location :type Vector))
  (AI|Navigation|SimpleMovetoLocation self Location)
  (Niagara|SpawnSystematLocation (Variables|Input|GetFXCursor) Location))

(fn Follow
  (params (Location :type Vector))
  (bind _returnvalue (Pawn|GetControlledPawn))
  (Pawn|Input|AddMovementInput _returnvalue (Math|Vector|GetUnitDirection(Vector) (Transformation|GetActorLocation _returnvalue) Location) 1.0 false))

(fn GetLocationUnderCursor
  (bind _hitresult (Game|Player|GetHitResultUnderCursorbyChannel "TraceTypeQuery1" true))
  (bind (_bblockinghit _binitialoverlap _time _distance _location) (Collision|BreakHitResult _hitresult))
  (return _bblockinghit _location))

(fn GetLocationUnderFinger
  (bind _hitresult (Class|PlayerController|GetHitResultUnderFingerbyChannel "Touch1" "TraceTypeQuery1" false))
  (bind (_bblockinghit _binitialoverlap _time _distance _location) (Collision|BreakHitResult _hitresult))
  (return _bblockinghit _location))

(fn InitCasts
  (bind _asbp_hud_spawn_tile (Utilities|Casting|CastToBP_HUD_SpawnTile (HUD|GetHUD)))
  (Variables|Default|SetAs%20BP%20HUD%20Spawn%20Tile _asbp_hud_spawn_tile))

(fn GetActorUnderCursor
  (bind _hitresult (Game|Player|GetHitResultUnderCursorbyChannel "TraceTypeQuery3" true))
  (bind (_bblockinghit _binitialoverlap _time _distance _location _impactpoint _normal _impactnormal _physmat _hitactor) (Collision|BreakHitResult _hitresult))
  (return _bblockinghit _hitactor))

(fn SetSelectedTile
  (params (SelectedActor :type Actor%20Object%20Reference))
  (Utilities|FlowControl|Sequence
    (:then_0
      (bind _asselectedactor (Variables|Default|GetAsSelectedActor)
        (:then
          (bind _asbp_actor_tile (Utilities|Casting|CastToBP_Actor_Tile _asselectedactor))
          (Default|RemovePlayerSelection _asbp_actor_tile self)
          (Variables|Default|SetAsSelectedActor 0))
        (:else)))
    (:then_1
      (bind _output_get (Variables|Default|SetAsSelectedActor SelectedActor))
      (bind _asbp_actor_tile_2 (Utilities|Casting|CastToBP_Actor_Tile _output_get))
      (Default|OnTileInteract _asbp_actor_tile_2 (Game|GetPlayerController 0)))))

(fn SelectActor
  (params (Actor :type Actor%20Object%20Reference))
  (Variables|Default|SetAsSelectedActor Actor))