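; BP_Pawn_Camera is a player camera pawn that can be panned around or snapped to a given actor.
; CameraMove feeds two input axes into movement input along the pawn's right and forward vectors.
; CameraFocus moves the pawn directly to a valid target actor's location without sweeping.
; Possession calls InitCasts, which is currently an empty stub.
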(event `self.ReceivePossessed`
  (params (NewController :type "Controller Object Reference"))
  (`self.InitCasts`))

(event `CameraMove`
  (params (InputAxisX :type "Float (double-precision)") (InputAxisY :type "Float (double-precision)"))
  (`self.AddMovementInput` (`self.GetActorRightVector`) InputAxisX)
  (`self.AddMovementInput` (`self.GetActorForwardVector`) InputAxisY))

(event `CameraFocus`
  (params (ActorToFocus :type "Actor Object Reference"))
  (`/Engine/EditorBlueprintResources/StandardMacros.IsValid` ActorToFocus
    (:`Is Valid`
      (`self.K2_SetActorLocation` self (`self.K2_GetActorLocation` ActorToFocus) false false))))

(fn `InitCasts`)

(fn `UserConstructionScript`)