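; Player controller for the SpawnTile game, handling camera movement, cursor selection of characters and spawn tiles, and Alive/Dead player status.
; Status changes swap the Interact and Dead Enhanced Input mapping contexts, starting as Dead.
; Select actions trace under the cursor on press, then notify the hit character or tile while clearing the previous selection.
; Keys 1 and 2 ask the GameMode to spawn a character or destroy the controlled one.
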(event `self.ReceiveBeginPlay`
  (bind _returnvalue (subsystem `EnhancedInputLocalPlayerSubsystem`))
  ;[0.05098 0.05098 0.05098] Add Mapping Context
  (`/Engine/EditorBlueprintResources/StandardMacros.IsValid` _returnvalue
    (:`Is Valid`
      (`EnhancedInputSubsystemInterface.AddMappingContext` _returnvalue "/Game/SpawnTile/Player/Input/IMC_Camera.IMC_Camera" 0 (struct))
      (`EnhancedInputSubsystemInterface.AddMappingContext` _returnvalue "/Game/SpawnTile/Player/Input/IMC_Interact.IMC_Interact" 0 (struct))
      (set `self.CurrentClickTraceChannel` "ECC_GameTraceChannel1")
      (set `self.bEnableClickEvents` true)
      (set `self.bEnableMouseOverEvents` true)
      (`self.UpdatePlayerControllerStatus` "NewEnumerator2"))))

(event `EventClientPostLogin`
  (if (`self.IsLocalPlayerController`)
    (bind _as_bp_hud_spawn_tile (`self.As BP HUD Spawn Tile`)
      (:`then`
        _)
      (:`else`
        (bind _asbp_hud_spawn_tile (cast `/Game/SpawnTile/HUD/BP_HUD_SpawnTile` (`self.GetHUD`)))
        (set `self.As BP HUD Spawn Tile` _asbp_hud_spawn_tile)))
    (`WidgetBlueprintLibrary.SetInputMode_GameAndUIEx` self (`/Game/SpawnTile/HUD/BP_HUD_SpawnTile.AsWBHUDSpawnTile` _as_bp_hud_spawn_tile))))

(event `EnhancedInput|/Game/SpawnTile/Player/Input/Actions/IA_Interact`
  (params (ActionValue :type Boolean) (ElapsedSeconds :type "Float (double-precision)") (TriggeredSeconds :type "Float (double-precision)") (InputAction :type "InputAction Object Reference" :default "/Game/SpawnTile/Player/Input/Actions/IA_Interact.IA_Interact"))
  (bind (_hit _hitactor) (`self.GetActorUnderCursorByChannel` "TraceTypeQuery3"))
  (:`Triggered`
    (bind _asinteractactor (`self.AsInteractActor`)
      (:`then`
        (if (`GameplayStatics.ObjectIsA` _asinteractactor "/Game/SpawnTile/Character/BP_Character_SpawnTile.BP_Character_SpawnTile_C")
          (`self.UpdateSelectedCharacter` (`self.AsInteractActor`))))
      (:`else`)))
  (:`Started`
    (if _hit
      (set `self.AsInteractActor` _hitactor)
      (else
        (set `self.AsInteractActor` null)
        (`self.UpdateSelectedCharacter` null)))))

(event `EnhancedInput|/Game/SpawnTile/Player/Input/Actions/IA_SelectSpawn`
  (params (ActionValue :type Boolean) (ElapsedSeconds :type "Float (double-precision)") (TriggeredSeconds :type "Float (double-precision)") (InputAction :type "InputAction Object Reference" :default "/Game/SpawnTile/Player/Input/Actions/IA_SelectSpawn.IA_SelectSpawn"))
  (bind (_hit _hitactor) (`self.GetActorUnderCursorByChannel` "TraceTypeQuery3"))
  (:`Triggered`
    (bind _asinteractactor (`self.AsInteractActor`)
      (:`then`
        (if (`GameplayStatics.ObjectIsA` _asinteractactor "/Game/SpawnTile/Tile/BP_Actor_Tile.BP_Actor_Tile_C")
          (`self.UpdateSelectedTile` (`self.AsInteractActor`))))
      (:`else`)))
  (:`Started`
    (`self.UpdateSelectedTile` null)
    (if _hit
      (set `self.AsInteractActor` _hitactor))))

(event `EnhancedInput|/Game/SpawnTile/Player/Input/Actions/IA_CameraMove`
  (params (ActionValue :type "Vector2D Structure") (ElapsedSeconds :type "Float (double-precision)") (TriggeredSeconds :type "Float (double-precision)") (InputAction :type "InputAction Object Reference" :default "/Game/SpawnTile/Player/Input/Actions/IA_CameraMove.IA_CameraMove"))
  (:`Triggered`
    (`self.As BP Pawn Camera`
      (:`then`
        _)
      (:`else`
        (bind _asbp_pawn_camera (cast `/Game/SpawnTile/Player/Camera/BP_Pawn_Camera` (`GameplayStatics.GetPlayerPawn` 0)))
        (set `self.As BP Pawn Camera` _asbp_pawn_camera)))
    (`/Game/SpawnTile/Player/Camera/BP_Pawn_Camera.CameraMove` (`self.As BP Pawn Camera`) ActionValue_X ActionValue_Y)))

(event `UpdatePlayerControllerStatus`
  (params (Selection :type "/Game/SpawnTile/System/Enum/E_PlayerStatus Enum" :default "NewEnumerator0"))
  (bind _output_get (set `self.PlayerStatus` Selection))
  (`self.OnStatusChanged` _output_get)
  (switch `/Game/SpawnTile/System/Enum/E_PlayerStatus` (`self.PlayerStatus`)
    (:`NewEnumerator1`
      (`EnhancedInputSubsystemInterface.RemoveMappingContext` (subsystem `EnhancedInputLocalPlayerSubsystem`) "/Game/SpawnTile/Player/Input/IMC_Dead.IMC_Dead" (struct))
      (`EnhancedInputSubsystemInterface.AddMappingContext` (subsystem `EnhancedInputLocalPlayerSubsystem`) "/Game/SpawnTile/Player/Input/IMC_Interact.IMC_Interact" 0 (struct)))
    (:`NewEnumerator2`
      (`EnhancedInputSubsystemInterface.RemoveMappingContext` (subsystem `EnhancedInputLocalPlayerSubsystem`) "/Game/SpawnTile/Player/Input/IMC_Interact.IMC_Interact" (struct))
      (`EnhancedInputSubsystemInterface.AddMappingContext` (subsystem `EnhancedInputLocalPlayerSubsystem`) "/Game/SpawnTile/Player/Input/IMC_Dead.IMC_Dead" 0 (struct)))))

(event `Key|One`
  (params (Key :type "Key Structure"))
  (:`Pressed`
    (`self.As BP GM Spawn Tiler`
      (:`then`
        _)
      (:`else`
        (bind _asbp_gm_spawn_tiler (cast `/Game/SpawnTile/Modes/BP_GM_SpawnTiler` (`GameplayStatics.GetGameMode`)))
        (set `self.As BP GM Spawn Tiler` _asbp_gm_spawn_tiler)))
    (`/Game/SpawnTile/Modes/BP_GM_SpawnTiler.EventSpawnCharacter` :`self` (`self.As BP GM Spawn Tiler`))))

(event `Key|Two`
  (params (Key :type "Key Structure"))
  (:`Pressed`
    (bind _ascontrolledcharacter (`self.AsControlledCharacter`)
      (:`then`
        (`self.K2_DestroyActor` _ascontrolledcharacter)
        (set `self.AsControlledCharacter` null)
        (`KismetSystemLibrary.PrintString` "Killed"))
      (:`else`
        (`KismetSystemLibrary.PrintString` "No Valid Character Ref")))))

(fn `GetActorUnderCursorByChannel`
  (params (TraceChannel :type "ETraceTypeQuery Enum" :default "TraceTypeQuery1"))
  (returns (Hit :type Boolean) (HitActor :type "Actor Object Reference"))
  (bind (_bblockinghit _binitialoverlap _time _distance _location _impactpoint _normal _impactnormal _physmat _hitactor) (`GameplayStatics.BreakHitResult` (`self.GetHitResultUnderCursorByChannel` TraceChannel)))
  (return _bblockinghit _hitactor))

(fn `InitCasts`
  (bind _asbp_ps_spawn_tile (cast `/Game/SpawnTile/Player/State/BP_PS_SpawnTile` (`GameplayStatics.GetPlayerState` 0))
    (:`then`
      (set `self.As BP PS Spawn Tile` _asbp_ps_spawn_tile)
      (bind _asbp_hud_spawn_tile (cast `/Game/SpawnTile/HUD/BP_HUD_SpawnTile` (`self.GetHUD`))
        (:`then`
          (set `self.As BP HUD Spawn Tile` _asbp_hud_spawn_tile)
          (bind _asbp_pawn_camera (cast `/Game/SpawnTile/Player/Camera/BP_Pawn_Camera` (`self.K2_GetPawn`))
            (:`then`
              (set `self.As BP Pawn Camera` _asbp_pawn_camera)
              (bind _asbp_gm_spawn_tiler (cast `/Game/SpawnTile/Modes/BP_GM_SpawnTiler` (`GameplayStatics.GetGameMode`))
                (:`then`
                  (set `self.As BP GM Spawn Tiler` _asbp_gm_spawn_tiler))
                (:`CastFailed`
                  (`KismetSystemLibrary.PrintString` "PC - GameMode Cast Failed"))))
            (:`CastFailed`
              (`KismetSystemLibrary.PrintString` "PC - Camera Cast Failed"))))
        (:`CastFailed`
          (`KismetSystemLibrary.PrintString` "PC - HUD Cast Failed"))))
    (:`CastFailed`
      (`KismetSystemLibrary.PrintString` "PC - PlayerState Cast Failed"))))

(fn `UpdateSelectedCharacter`
  (params (Actor :type "Actor Object Reference"))
  (`/Engine/EditorBlueprintResources/StandardMacros.IsValid` Actor
    (:`Is Valid`
      (bind _asselectedcharacter (`self.AsSelectedCharacter`)
        (:`then`
          (`/Game/SpawnTile/Character/BP_Character_SpawnTile.EventActorEndInteract` _asselectedcharacter))
        (:`else`
          _))
      (bind _asbp_character_spawn_tile (cast `/Game/SpawnTile/Character/BP_Character_SpawnTile` Actor))
      (bind _output_get (set `self.AsSelectedCharacter` _asbp_character_spawn_tile))
      (`/Game/SpawnTile/Character/BP_Character_SpawnTile.EventActorBeginInteract` _output_get))
    (:`Is Not Valid`
      (bind _asselectedcharacter_2 (`self.AsSelectedCharacter`)
        (:`then`
          (`/Game/SpawnTile/Character/BP_Character_SpawnTile.EventActorEndInteract` _asselectedcharacter_2))
        (:`else`)))))

(fn `UpdateSelectedTile`
  (params (InteractActor :type "Actor Object Reference"))
  (`|ExecutionSequence`
    (:`then_0`
      (bind _as_selected_bp_actor_tile (`self.As Selected BP Actor Tile`)
        (:`then`
          (`/Game/SpawnTile/Tile/BP_Actor_Tile.RemovePlayerSelection` _as_selected_bp_actor_tile self))
        (:`else`)))
    (:`then_1`
      (bind _asbp_actor_tile (cast `/Game/SpawnTile/Tile/BP_Actor_Tile` InteractActor))
      (bind _output_get (set `self.As Selected BP Actor Tile` _asbp_actor_tile))
      (`/Game/SpawnTile/Tile/BP_Actor_Tile.EventOnTileInteract` _output_get (`GameplayStatics.GetPlayerController` 0)))))

(fn `UserConstructionScript`)