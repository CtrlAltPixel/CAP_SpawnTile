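; Gameplay player controller for tile selection, pawn camera movement and the HUD dead overlay.
; On local BeginPlay it initializes camera, HUD and tile mode through Enhanced Input contexts; interact init is never called.
; Cursor-trace clicks toggle or switch the selected tile, adding or removing the PlayerState through Local/Server event pairs.
; Debug keys ask the GameMode to spawn a unit and the GameState to resolve.
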(event EventBeginPlay
  (if (Pawn|IsLocalPlayerController)
    (Utilities|FlowControl|Sequence
      (:then_0
        (if (Variables|Debug|GetbShowDebug?)
          (Development|PrintString "BP_PC_Gameplay - EVENT BeginPlay" true true "(R=0.000000,G=0.660000,B=1.000000,A=1.000000)" 3.0)))
      (:then_1
        (CallFunction|EventPlayerControllerInitCamera)
        (CallFunction|EventPlayerControllerInitHUD)
        (Variables|Default|SetbShowMouseCursor true)
        (Variables|Default|SetbEnableClickEvents true)
        (Variables|Default|SetbEnableMouseOverEvents true)
        (CallFunction|EventPlayerControllerInitTile)))))

(event Input|KeyboardEvents|DebugKey1
  (params (Key :type Key%20Structure) (ActionValue :type Input%20Action%20Value%20Structure)))

(event Input|KeyboardEvents|DebugKey2
  (params (Key :type Key%20Structure) (ActionValue :type Input%20Action%20Value%20Structure)))

(event Custom|EventPlayerControllerInitCamera
  (bind _returnvalue (PlayerController|LocalPlayerSubsystems|GetEnhancedInputLocalPlayerSubsystem))
  (Utilities|FlowControl|Sequence
    (:then_0
      (if (Variables|Debug|GetbShowDebug?)
        (Development|PrintString "BP_PC_Gameplay - EVENT Init Camera" true true "(R=0.000000,G=0.660000,B=1.000000,A=1.000000)" 3.0)))
    (:then_1
      (Utilities|IsValid _returnvalue
        (:Is%20Valid
          (Input|AddMappingContext _returnvalue "/Game/SpawnTile/Player/Input/IMC_Camera.IMC_Camera" 0 "(bIgnoreAllPressedKeysUntilRelease=True,bForceImmediately=False,bNotifyUserSettings=False)")
          (Variables|Reference|GetAs%20BP%20Pawn%20Camera
            (:then
              (Actor|DestroyActor (Variables|Reference|GetAs%20BP%20Pawn%20Camera)))
            (:else
              _))
          (bind _asbp_pawn_camera (Utilities|Casting|CastToBP_Pawn_Camera (Pawn|GetControlledPawn))
            (:then
              (Variables|Reference|SetAs%20BP%20Pawn%20Camera _asbp_pawn_camera))
            (:CastFailed
              (if (Variables|Debug|GetbShowDebug?)
                (Development|PrintString "BP_PC_Gameplay - EVENT Init Camera FAILED to cast to BP_Pawn_Camera" true true "(R=0.000000,G=0.660000,B=1.000000,A=1.000000)" 3.0)))))
        (:Is%20Not%20Valid
          (if (Variables|Debug|GetbShowDebug?)
            (Development|PrintString "BP_PC_Gameplay - EVENT Init Camera INVALID Enhanced Input Subsytem" true true "(R=0.000000,G=0.660000,B=1.000000,A=1.000000)" 3.0)))))))

(event Input|EnhancedActionEvents|EnhancedInputActionIA_Camera_Move
  (params (ActionValue :type Vector%202D%20Structure) (ElapsedSeconds :type Float%20%28double-precision%29) (TriggeredSeconds :type Float%20%28double-precision%29) (InputAction :type Input%20Action%20Object%20Reference :default "/Game/SpawnTile/Player/Input/Actions/Camera/IA_Camera_Move.IA_Camera_Move"))
  (bind _as_bp_pawn_camera (Variables|Reference|GetAs%20BP%20Pawn%20Camera)
    (:then
      (Default|CameraMove _as_bp_pawn_camera (.x ActionValue) (.y ActionValue)))
    (:else)))

(event Custom|EventPlayerControllerInitInteract
  (bind _returnvalue (PlayerController|LocalPlayerSubsystems|GetEnhancedInputLocalPlayerSubsystem))
  (Utilities|FlowControl|Sequence
    (:then_0
      (if (Variables|Debug|GetbShowDebug?)
        (Development|PrintString "BP_PC_Gameplay - EVENT Init Interact" true true "(R=0.000000,G=0.660000,B=1.000000,A=1.000000)" 3.0)))
    (:then_1
      (Utilities|IsValid _returnvalue
        (:Is%20Valid
          (Input|AddMappingContext _returnvalue "/Game/SpawnTile/Player/Input/IMC_Interact.IMC_Interact" 0 "(bIgnoreAllPressedKeysUntilRelease=True,bForceImmediately=False,bNotifyUserSettings=False)")
          (Variables|Default|SetCurrentClickTraceChannel "ECC_GameTraceChannel1"))))))

(event Custom|EventPlayerControllerInitUnit
  (params (AsControlledCharacter :type BP%20Character%20Player%20Object%20Reference))
  (Variables|Reference|GetAs%20BP%20Character%20Unit
    (:then
      (Actor|DestroyActor (Variables|Reference|GetAs%20BP%20Character%20Unit)))
    (:else
      _))
  (Variables|Reference|SetAs%20BP%20Character%20Unit AsControlledCharacter))

(event Custom|EventPlayerControllerUpdateUnitState
  (params (UnitState :type E_UnitState%20Enum :default "NewEnumerator0"))
  (Utilities|FlowControl|Sequence
    (:then_0
      (if (Variables|Debug|GetbShowDebug?)
        (Development|PrintString "BP_PS_Gameplay - EVENT Update Unit State" true true "(R=0.000000,G=0.660000,B=1.000000,A=1.000000)" 3.0)))
    (:then_1
      (Variables|Default|SetUnitState UnitState))))

(event Custom|EventPlayerControllerInitTile
  (bind _returnvalue (PlayerController|LocalPlayerSubsystems|GetEnhancedInputLocalPlayerSubsystem))
  (Utilities|FlowControl|Sequence
    (:then_0
      (if (Variables|Debug|GetbShowDebug?)
        (Development|PrintString "BP_PC_Gameplay - EVENT Init Tile" true true "(R=0.000000,G=0.660000,B=1.000000,A=1.000000)" 3.0)))
    (:then_1
      (Utilities|IsValid _returnvalue
        (:Is%20Valid
          (Input|AddMappingContext _returnvalue "/Game/SpawnTile/Player/Input/IMC_Tile.IMC_Tile" 0 "(bIgnoreAllPressedKeysUntilRelease=True,bForceImmediately=False,bNotifyUserSettings=False)")
          (Input|RemoveMappingContext _returnvalue "/Game/SpawnTile/Player/Input/IMC_Interact.IMC_Interact" "(bIgnoreAllPressedKeysUntilRelease=True,bForceImmediately=False,bNotifyUserSettings=False)")
          (Variables|Default|SetCurrentClickTraceChannel "ECC_GameTraceChannel2"))))))

(event Custom|EventPlayerControllerAddPlayerStateServer
  (params (Tile :type BP%20Actor%20Tile%20Object%20Reference) (PlayerState :type Player%20State%20Object%20Reference))
  (Utilities|IsValid Tile
    (:Is%20Valid
      (Default|EventTilePlayerStateAdd Tile PlayerState))))

(event Custom|EventPlayerControllerRemovePlayerStateServer
  (params (PlayerState :type Player%20State%20Object%20Reference))
  (Utilities|FlowControl|Sequence
    (:then_0
      (if (Variables|Debug|GetbShowDebug?)
        (Development|PrintString "BP_PC_Gameplay - EVENT Remove PlayerState On Server" true true "(R=0.000000,G=0.660000,B=1.000000,A=1.000000)" 3.0)))
    (:then_1
      (bind _as_bp_actor_tile (Variables|Reference|GetAs%20BP%20Actor%20Tile)
        (:then
          (Default|EventTilePlayerStateRemove _as_bp_actor_tile PlayerState))
        (:else)))))

(event Custom|EventPlayerControllerAddPlayerStateLocal
  (params (Actor :type Actor%20Object%20Reference))
  (Variables|Reference|GetAs%20BP%20Actor%20Tile
    (:then
      (CallFunction|EventPlayerControllerRemovePlayerStateLocal))
    (:else
      _))
  (bind _asbp_actor_tile (Utilities|Casting|CastToBP_Actor_Tile Actor))
  (bind _output_get (Variables|Reference|SetAs%20BP%20Actor%20Tile _asbp_actor_tile))
  (CallFunction|EventPlayerControllerAddPlayerStateServer _output_get (Variables|/Script/Engine.Controller|GetPlayerState (Game|GetPlayerController 0))))

(event Custom|EventPlayerControllerRemovePlayerStateLocal
  (Utilities|FlowControl|Sequence
    (:then_0
      (if (Variables|Debug|GetbShowDebug?)
        (Development|PrintString "BP_PC_Gameplay - EVENT Remove PlayerState Local" true true "(R=0.000000,G=0.660000,B=1.000000,A=1.000000)" 3.0)))
    (:then_1
      (Variables|Reference|GetAs%20BP%20Actor%20Tile
        (:then
          (CallFunction|EventPlayerControllerRemovePlayerStateServer (Variables|/Script/Engine.Controller|GetPlayerState (Game|GetPlayerController 0)))
          (Variables|Reference|SetAs%20BP%20Actor%20Tile 0))
        (:else)))))

(event Input|EnhancedActionEvents|EnhancedInputActionIA_Tile_Primary
  (params (ActionValue :type Boolean) (ElapsedSeconds :type Float%20%28double-precision%29) (TriggeredSeconds :type Float%20%28double-precision%29) (InputAction :type Input%20Action%20Object%20Reference :default "/Game/SpawnTile/Player/Input/Actions/Tile/IA_Tile_Primary.IA_Tile_Primary"))
  (bind (_hit _hitactor) (CallFunction|GetActorUnderCursorbyChannel "TraceTypeQuery4"))
  (:Started
    (if _hit
      (bind _as_bp_actor_tile (Variables|Reference|GetAs%20BP%20Actor%20Tile)
        (:then
          (if (== _as_bp_actor_tile _hitactor)
            (CallFunction|EventPlayerControllerRemovePlayerStateLocal)
            (else
              (CallFunction|EventPlayerControllerRemovePlayerStateLocal)
              (CallFunction|EventPlayerControllerAddPlayerStateLocal _hitactor))))
        (:else
          (CallFunction|EventPlayerControllerAddPlayerStateLocal _hitactor))))))

(event Input|EnhancedActionEvents|EnhancedInputActionIA_Tile_Secondary
  (params (ActionValue :type Boolean) (ElapsedSeconds :type Float%20%28double-precision%29) (TriggeredSeconds :type Float%20%28double-precision%29) (InputAction :type Input%20Action%20Object%20Reference :default "/Game/SpawnTile/Player/Input/Actions/Tile/IA_Tile_Secondary.IA_Tile_Secondary"))
  (:Started
    (Utilities|FlowControl|Sequence
      (:then_0
        (if (Variables|Debug|GetbShowDebug?)
          (Development|PrintString "BP_PC_Gameplay - EVENT Cancel Tile On SERVER" true true "(R=0.000000,G=0.660000,B=1.000000,A=1.000000)" 3.0)))
      (:then_1
        (CallFunction|EventPlayerControllerRemovePlayerStateLocal)))))

(event Input|KeyboardEvents|DebugKey4
  (params (Key :type Key%20Structure :default "None") (ActionValue :type Input%20Action%20Value%20Structure))
  (:Pressed
    (Variables|Reference|GetAs%20BP%20GM%20Gameplay
      (:then
        _)
      (:else
        (bind _asbp_gm_gameplay (Utilities|Casting|CastToBP_GM_Gameplay (Game|GetGameMode)))
        (Variables|Reference|SetAs%20BP%20GM%20Gameplay _asbp_gm_gameplay)))
    (Default|EventGameModeSpawnPlayerUnit (Variables|Reference|GetAs%20BP%20GM%20Gameplay) (Variables|/Script/Engine.Controller|GetPlayerState (Game|GetPlayerController 0)))))

(event Input|KeyboardEvents|DebugKey5
  (params (Key :type Key%20Structure :default "None") (ActionValue :type Input%20Action%20Value%20Structure))
  (:Pressed
    (Variables|Reference|GetAs%20BP%20GS%20Gameplay
      (:then
        _)
      (:else
        (bind _asbp_gs_gameplay (Utilities|Casting|CastToBP_GS_Gameplay (Game|GetGameState)))
        (Variables|Reference|SetAs%20BP%20GS%20Gameplay _asbp_gs_gameplay)))
    (Default|EventGameStateResolve (Variables|Reference|GetAs%20BP%20GS%20Gameplay))))

(event Custom|EventPlayerControllerInitHUD
  (Utilities|FlowControl|Sequence
    (:then_0
      (if (Variables|Debug|GetbShowDebug?)
        (Development|PrintString "BP_PS_Gameplay - EVENT Init HUD" true true "(R=0.000000,G=0.660000,B=1.000000,A=1.000000)" 3.0)))
    (:then_1
      (bind _asbp_hud_gameplay (Utilities|Casting|CastToBP_HUD_Gameplay (HUD|GetHUD)))
      (Variables|Reference|SetAs%20BP%20HUD%20Gameplay _asbp_hud_gameplay))))

(event Custom|EventPlayerControllerUpdateHUDCharacterState
  (params (UnitState :type E_UnitState%20Enum :default "NewEnumerator0"))
  (Utilities|FlowControl|Sequence
    (:then_0
      (if (Variables|Debug|GetbShowDebug?)
        (Development|PrintString "BP_PS_Gameplay - EVENT IUpdate HUD State" true true "(R=0.000000,G=0.660000,B=1.000000,A=1.000000)" 3.0)))
    (:then_1
      (Variables|Reference|GetAs%20BP%20HUD%20Gameplay
        (:then
          (switch Utilities|FlowControl|Switch|SwitchonE_UnitState UnitState
            (:NewEnumerator1
              (Default|EventHUDHideDeadOverlay (Variables|Reference|GetAs%20BP%20HUD%20Gameplay)))
            (:NewEnumerator2
              (Default|EventHUDShowDeadOverlay (Variables|Reference|GetAs%20BP%20HUD%20Gameplay)))))
        (:else)))))

(fn ConstructionScript)

(fn GetActorUnderCursorbyChannel
  (params (TraceChannel :type ETraceTypeQuery%20Enum :default "TraceTypeQuery1"))
  (bind _hitresult (Game|Player|GetHitResultUnderCursorbyChannel TraceChannel true))
  (bind (_bblockinghit _binitialoverlap _time _distance _location _impactpoint _normal _impactnormal _physmat _hitactor) (Collision|BreakHitResult _hitresult))
  (return _bblockinghit _hitactor))