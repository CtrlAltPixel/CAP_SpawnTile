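; Game state for the SpawnTile mode that runs turn-based spawning on a looping timer, started shortly after BeginPlay.
; Turn start increments and prints TurnCount, then asks the game mode to spawn a character for each player state with a spawn set.
; Turn end clears each player's spawn action through a server call.
; TurnCount's OnRep fires an update dispatcher with the new count.
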(event `self.ReceiveBeginPlay`
  (`KismetSystemLibrary.Delay` 3.0)
  (`self.EventMatchStart`))

(event `EventMatchStart`
  (bind _returnvalue (`KismetSystemLibrary.K2_SetTimerDelegate` (`|CreateDelegate` :!event `EventTurnStart`) 7.0 true))
  (set `self.TurnTimer` _returnvalue))

(event `EventTurnStart`
  (`self.UpdateTurnCount`)
  (for _array_element (`self.PlayerArray`)
    (bind _asbp_ps_spawn_tile (cast `/Game/SpawnTile/Player/State/BP_PS_SpawnTile` _array_element))
    (if (`/Game/SpawnTile/Player/State/BP_PS_SpawnTile.IsSpawnSet?` _asbp_ps_spawn_tile)
      (bind _asbp_gm_spawn_tiler (cast `/Game/SpawnTile/Modes/BP_GM_SpawnTiler` (`GameplayStatics.GetGameMode`)))
      (`/Game/SpawnTile/Modes/BP_GM_SpawnTiler.EventSpawnCharacter` _asbp_gm_spawn_tiler (`PlayerState.GetPlayerController` _asbp_ps_spawn_tile) (`/Game/SpawnTile/Player/State/BP_PS_SpawnTile.SpawnTransform` _asbp_ps_spawn_tile)))))

(event `EventTurnEnd`
  (for _array_element (`self.PlayerArray`)
    (bind _asbp_ps_spawn_tile (cast `/Game/SpawnTile/Player/State/BP_PS_SpawnTile` _array_element))
    (`/Game/SpawnTile/Player/State/BP_PS_SpawnTile.SERVER_UpdateActionSpawn` :`self` _asbp_ps_spawn_tile)))

(fn `OnRep_TurnCount`
  (`self.OnUpdateTurnCount` (`self.TurnCount`)))

(fn `UpdateTurnCount`
  (bind _output_get (set `self.TurnCount` (+ (`self.TurnCount`) 1)))
  (`KismetSystemLibrary.PrintString` (`KismetStringLibrary.Concat_StrStr` "Turn:" (`KismetStringLibrary.Conv_IntToString` _output_get))))

(fn `UserConstructionScript`)