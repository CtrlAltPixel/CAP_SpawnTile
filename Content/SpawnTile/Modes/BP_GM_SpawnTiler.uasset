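; Game mode for SpawnTile that spawns player characters on request and tracks connected player controllers.
; Spawning links the new character to its controller, updates that controller's status and clears the spawn action on its player state.
; A died-character event clears the controller's character reference and updates its status.
; Login and logout maintain the controller list, with login also calling the controller's client post-login event.
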(event `self.ReceiveBeginPlay`
  ; Set Game Instance "StartGame Offset" (Float) from game instance get game time in seconds (Custom Var)
  (`KismetSystemLibrary.PrintString` "Game Mode")
  (add `self.OnPlayerDied` (`|CreateDelegate` :!event `EventCharacterDied`)))

(event `EventCharacterDied` :!signature `self.OnPlayerDied`
  (params (Character :type "Character Object Reference"))
  (bind _asbp_character_player (cast `/Game/SpawnTile/Character/Player/BP_Character_Player` Character))
  (bind _asbp_pc_spawn_tile (cast `/Game/SpawnTile/Player/Controller/BP_PC_SpawnTile` (`/Game/SpawnTile/Character/BP_Character_SpawnTile.CommandController` _asbp_character_player)))
  (set `/Game/SpawnTile/Player/Controller/BP_PC_SpawnTile.AsControlledCharacter` null _asbp_pc_spawn_tile)
  (`/Game/SpawnTile/Player/Controller/BP_PC_SpawnTile.UpdatePlayerControllerStatus` _asbp_pc_spawn_tile "NewEnumerator2"))

(event `EventSpawnCharacter`
  (params (Playercontroller :type "PlayerController Object Reference") (SpawnTransform :type "Transform Structure"))
  (`/Engine/EditorBlueprintResources/StandardMacros.IsValid` Playercontroller
    (:`Is Valid`
      (bind _returnvalue (`|SpawnActorFromClass` "/Game/SpawnTile/Character/Player/BP_Character_Player.BP_Character_Player_C" SpawnTransform "Undefined" "MultiplyWithRoot" null Playercontroller "NewEnumerator1" null))
      (bind _asbp_pc_spawn_tile (cast `/Game/SpawnTile/Player/Controller/BP_PC_SpawnTile` Playercontroller))
      (set `/Game/SpawnTile/Player/Controller/BP_PC_SpawnTile.AsControlledCharacter` _returnvalue _asbp_pc_spawn_tile)
      (`/Game/SpawnTile/Player/Controller/BP_PC_SpawnTile.UpdatePlayerControllerStatus` _asbp_pc_spawn_tile "NewEnumerator1")
      (bind _asbp_ps_spawn_tile (cast `/Game/SpawnTile/Player/State/BP_PS_SpawnTile` (`Controller.PlayerState` Playercontroller)))
      (`/Game/SpawnTile/Player/State/BP_PS_SpawnTile.SERVER_UpdateActionSpawn` :`self` _asbp_ps_spawn_tile))))

(event `self.K2_PostLogin`
  (params (NewPlayer :type "PlayerController Object Reference"))
  (`KismetArrayLibrary.Array_Add` (`self.AllPlayerControllers`) NewPlayer)
  (bind _asbp_pc_spawn_tile (cast `/Game/SpawnTile/Player/Controller/BP_PC_SpawnTile` NewPlayer))
  (`/Game/SpawnTile/Player/Controller/BP_PC_SpawnTile.EventClientPostLogin` _asbp_pc_spawn_tile))

(event `self.K2_OnLogout`
  (params (ExitingController :type "Controller Object Reference"))
  (bind _asplayer_controller (cast `PlayerController` ExitingController))
  (`KismetArrayLibrary.Array_RemoveItem` (`self.AllPlayerControllers`) _asplayer_controller))

(fn `UserConstructionScript`)