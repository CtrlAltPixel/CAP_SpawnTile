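; Gameplay game state Blueprint that scaffolds a turn-based match as chained start/end events, with optional debug prints.
; Match start fires after a BeginPlay delay but only reaches a print-only timer event, with no call into the turn loop.
; Each turn runs timed planning, then an empty spawn phase, repeating until the turn limit ends the match.
; Input toggling and action queue functions are empty stubs.
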(event `self.ReceiveBeginPlay`
  (`KismetSystemLibrary.Delay` 3.0)
  (`self.EventGameStateMatchStart`))

(event `EventGameStateMatchStart`
  (`|ExecutionSequence`
    (:`then_0`
      (if (`self.bShowDebug?`)
        (`KismetSystemLibrary.PrintString` "BP_GS_Gameplay - EVENT Match Start" true true (struct :`G` 0.66 :`B` 1.0 :`A` 1.0) 3.0)))
    (:`then_1`
      (`self.EventGameStateTimerStart`))))

(event `EventGameStateMatchEnd`
  (`|ExecutionSequence`
    (:`then_0`
      (if (`self.bShowDebug?`)
        (`KismetSystemLibrary.PrintString` "BP_GS_Gameplay - EVENT MatchEnd" true true (struct :`G` 0.66 :`B` 1.0 :`A` 1.0) 3.0)))
    (:`then_1`
      (`self.EventGameStateTimerEnd`))))

(event `EventGameStateTimerStart`
  (`|ExecutionSequence`
    (:`then_0`
      (if (`self.bShowDebug?`)
        (`KismetSystemLibrary.PrintString` "BP_GS_Gameplay - EVENT Timer Start" true true (struct :`G` 0.66 :`B` 1.0 :`A` 1.0) 3.0)))))

(event `EventGameStateTimerEnd`
  (`|ExecutionSequence`
    (:`then_0`
      (if (`self.bShowDebug?`)
        (`KismetSystemLibrary.PrintString` "BP_GS_Gameplay - EVENT Timer End" true true (struct :`G` 0.66 :`B` 1.0 :`A` 1.0) 3.0)))))

(event `EventGameStateTurnStart`
  (`|ExecutionSequence`
    (:`then_0`
      (if (`self.bShowDebug?`)
        (`KismetSystemLibrary.PrintString` "BP_GS_Gameplay - EVENT Turn Start" true true (struct :`G` 0.66 :`B` 1.0 :`A` 1.0) 3.0)))
    (:`then_1`
      (set `self.TurnCount` (+ (`self.TurnCount`) 1))
      (`self.EventGameStatePlanningStart`))))

(event `EventGameStateTurnEnd`
  (`|ExecutionSequence`
    (:`then_0`
      (if (`self.bShowDebug?`)
        (`KismetSystemLibrary.PrintString` "BP_GS_Gameplay - EVENT Turn End" true true (struct :`G` 0.66 :`B` 1.0 :`A` 1.0) 3.0)))
    (:`then_1`
      (bind _returnvalue (`self.Func_IsMaxTurn?`))
      (if _returnvalue
        (`self.EventGameStateMatchEnd`)
        (else
          (`self.EventGameStateTurnStart`))))))

(event `EventGameStatePlanningStart`
  (`|ExecutionSequence`
    (:`then_0`
      (if (`self.bShowDebug?`)
        (`KismetSystemLibrary.PrintString` "BP_GS_Gameplay - EVENT PlanningStart")))
    (:`then_1`
      (`self.Func_EnableInput`)
      (`self.EventGameStateCountdownStart` 5.0))))

(event `EventGameStateCountdownStart`
  (params (Time :type "Float (single-precision)"))
  (`|ExecutionSequence`
    (:`then_0`
      (if (`self.bShowDebug?`)
        (`KismetSystemLibrary.PrintString` "BP_GS_Gameplay - EVENT Countdown Start" true true (struct :`G` 0.66 :`B` 1.0 :`A` 1.0) 3.0)))
    (:`then_1`
      (bind _returnvalue (`KismetSystemLibrary.K2_SetTimerDelegate` (`|CreateDelegate` :!event `EventGameStateCountdownEnd`) Time))
      (set `self.PlanningTimer` _returnvalue))))

(event `EventGameStateCountdownEnd`
  (`|ExecutionSequence`
    (:`then_0`
      (if (`self.bShowDebug?`)
        (`KismetSystemLibrary.PrintString` "BP_GS_Gameplay - EVENT Countdown Stop" true true (struct :`G` 0.66 :`B` 1.0 :`A` 1.0) 3.0)))
    (:`then_1`
      (`KismetSystemLibrary.K2_ClearAndInvalidateTimerHandle` (`self.PlanningTimer`))
      (`self.EventGameStatePlanningEnd`))))

(event `EventGameStatePlanningEnd`
  (`|ExecutionSequence`
    (:`then_0`
      (if (`self.bShowDebug?`)
        (`KismetSystemLibrary.PrintString` "BP_GS_Gameplay - EVENT Planning End")))
    (:`then_1`
      (`self.Func_DisableInput`)
      (`self.EventGameStateSpawnStart`))))

(event `EventGameStateSpawnStart`
  (`|ExecutionSequence`
    (:`then_0`
      (if (`self.bShowDebug?`)
        (`KismetSystemLibrary.PrintString` "BP_GS_Gameplay - EVENT SpawnStart")))
    (:`then_1`
      (`self.eventGameStateSpawnEnd`))))

(event `EventGameStateSpawnEnd`
  (`|ExecutionSequence`
    (:`then_0`
      (if (`self.bShowDebug?`)
        (`KismetSystemLibrary.PrintString` "BP_GS_Gameplay - EVENT Spawn End")))
    (:`then_1`
      (`self.EventGameStateTurnEnd`))))

(fn `Func_CreateActionQue`)

(fn `Func_DisableInput`)

(fn `Func_EnableInput`)

(fn `Func_IsMaxTurn?`
  (returns (ReturnValue :type Boolean))
  (return (>= (`self.TurnCount`) 10)))

(fn `UserConstructionScript`)