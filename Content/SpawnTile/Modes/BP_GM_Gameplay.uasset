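; Gameplay game mode that tracks connected PlayerControllers and spawns player units on spawn tiles.
; PostLogin and OnLogout maintain the controller list.
; The spawn event creates a BP_Character_Player at the tile, passing the requesting player as CommandPlayerController, then has a new BP_AIController_SpawnTile possess it.
; BeginPlay binds to OnPlayerDied, while the character-death handler is a stub that only casts to the player character.
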(event `self.ReceiveBeginPlay`
  (add `self.OnPlayerDied` (`|CreateDelegate` :!event `EventCharacterDied`)))

(event `self.K2_PostLogin`
  (params (NewPlayer :type "PlayerController Object Reference"))
  (`KismetArrayLibrary.Array_Add` (`self.AllPlayerControllers`) NewPlayer))

(event `self.K2_OnLogout`
  (params (ExitingController :type "Controller Object Reference"))
  (bind _asplayer_controller (cast `PlayerController` ExitingController))
  (`KismetArrayLibrary.Array_RemoveItem` (`self.AllPlayerControllers`) _asplayer_controller))

(event `EventGameModeSpawnPlayerUnit`
  (params (SpawnTile :type "/Game/SpawnTile/Tile/BP_Actor_Tile Object Reference") (`Player Controller` :type "PlayerController Object Reference"))
  (bind _returnvalue (`self.GetTransform` SpawnTile))
  (`|ExecutionSequence`
    (:`then_0`
      (if (`self.bShowDebug?`)
        (`KismetSystemLibrary.PrintString` "BP_GM_Gameplay - EVENT Spawn Player Unit" true true (struct :`G` 0.66 :`B` 1.0 :`A` 1.0) 3.0)))
    (:`then_1`
      (bind _returnvalue_2 (`|SpawnActorFromClass` "/Game/SpawnTile/Character/Player/BP_Character_Player.BP_Character_Player_C" _returnvalue "Undefined" "MultiplyWithRoot" null `Player Controller` "NewEnumerator1" null))
      (bind _returnvalue_3 (`|SpawnActorFromClass` "/Game/SpawnTile/Character/AI/BP_AIController_SpawnTile.BP_AIController_SpawnTile_C" _returnvalue "Undefined" "MultiplyWithRoot" null null))
      (`Controller.Possess` _returnvalue_3 _returnvalue_2))))

(event `EventCharacterDied` :!signature `self.OnPlayerDied`
  (params (Character :type "Character Object Reference"))
  (`|ExecutionSequence`
    (:`then_0`
      (if (`self.bShowDebug?`)
        _))
    (:`then_1`
      (cast `/Game/SpawnTile/Character/Player/BP_Character_Player` Character))))

(fn `UserConstructionScript`)